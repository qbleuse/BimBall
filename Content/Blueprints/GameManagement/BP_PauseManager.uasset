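; Pause manager actor that toggles game pause and drives the BP_PauseMenuUI widget through gamepad-style input actions.
; ActivatePause flip-flops pause, swapping input between itself and the player character and animating the menu in or out.
; Wrapping selection indices handle resume, restart, settings and return-to-hub, plus settings tabs for video, volume and controls.
; The widget handles display and most settings changes, while BP_BimBallGameMode handles level loading and camera-axis inversion.
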(event Custom|ActivatePause
  (bind _returnvalue (Game|GetPlayerCharacter 0))
  (bind _returnvalue_2 (Game|GetPlayerController 0))
  (bind _pausemenu (Variables|Default|GetPauseMenu))
  ;[1 1 1] ActivatePause
  (bind _isa (Utilities|FlowControl|FlipFlop)
    (:A
      (Game|SetGamePaused _isa)
      (UserInterface|Viewport|AddtoViewport (Variables|Default|GetPauseMenu) 0)
      (Input|EnableInput _returnvalue_2)
      (Input|DisableInput _returnvalue _returnvalue_2)
      (Variables|Default|SetSelectedOption 0)
      (Variables|Default|SetInSettings false)
      (Variables|Default|SetSelectedTab 0)
      (Default|OpenPauseMenu _pausemenu "Forward" (Variables|Default|GetSelectedOption) (Variables|Default|GetSelectedTab)))
    (:B
      (Game|SetGamePaused _isa)
      (Input|DisableInput _returnvalue_2)
      (Input|EnableInput _returnvalue _returnvalue_2)
      (if (Variables|Default|GetInSettings)
        (Utilities|FlowControl|Sequence
          (:then_0
            (CallFunction|OpenSettings))
          (:then_1
            (Default|OpenPauseMenu _pausemenu "Reverse" (Variables|Default|GetSelectedOption) (Variables|Default|GetSelectedTab) :!label _label)
            (Utilities|FlowControl|Delay (Class|WidgetAnimation|GetEndTime (Variables|/Game/Blueprints/UI/Menus/BP_PauseMenuUI.BP_PauseMenuUI_C|GetPlayingAnimation _pausemenu)))
            (Widget|RemovefromParent _pausemenu)))
        (else
          (goto _label))))))

(event Custom|OpenSettings
  ;[1 1 1] OpenSettings
  (bind _isa (Utilities|FlowControl|FlipFlop)
    (:A
      _)
    (:B
      _))
  (Variables|Default|SetInSettings _isa)
  (Default|OpenSettingsPanel (Variables|Default|GetPauseMenu) (select _isa "Forward" "Reverse") _isa))

(event EventBeginPlay
  ;[1 1 1] CreateWidget
  (Class|Actor|SetTickablewhenPaused true)
  (Input|DisableInput (Game|GetPlayerController 0))
  (bind _returnvalue (UserInterface|CreateWidget "/Game/Blueprints/UI/Menus/BP_PauseMenuUI.BP_PauseMenuUI_C"))
  (Variables|Default|SetPauseMenu _returnvalue)
  (bind _asbp_bim_ball_game_mode (Utilities|Casting|CastToBP_BimBallGameMode (Game|GetGameMode)))
  (Variables|Default|SetGameMode _asbp_bim_ball_game_mode))

(event Input|ActionEvents|InputActionQuit
  (params (Key :type Key%20Structure :default "None"))
  (bind _returnvalue (Game|GetPlayerCharacter 0))
  (bind _returnvalue_2 (Game|GetPlayerController 0))
  (bind _pausemenu (Variables|Default|GetPauseMenu))
  ;[1 1 1] ActivatePause
  (:Pressed
    (bind _isa (Utilities|FlowControl|FlipFlop)
      (:A
        (Game|SetGamePaused _isa)
        (UserInterface|Viewport|AddtoViewport (Variables|Default|GetPauseMenu) 0)
        (Input|EnableInput _returnvalue_2)
        (Input|DisableInput _returnvalue _returnvalue_2)
        (Variables|Default|SetSelectedOption 0)
        (Variables|Default|SetInSettings false)
        (Variables|Default|SetSelectedTab 0)
        (Default|OpenPauseMenu _pausemenu "Forward" (Variables|Default|GetSelectedOption) (Variables|Default|GetSelectedTab)))
      (:B
        (Game|SetGamePaused _isa)
        (Input|DisableInput _returnvalue_2)
        (Input|EnableInput _returnvalue _returnvalue_2)
        (if (Variables|Default|GetInSettings)
          (Utilities|FlowControl|Sequence
            (:then_0
              (CallFunction|OpenSettings))
            (:then_1
              (Default|OpenPauseMenu _pausemenu "Reverse" (Variables|Default|GetSelectedOption) (Variables|Default|GetSelectedTab) :!label _label)
              (Utilities|FlowControl|Delay (Class|WidgetAnimation|GetEndTime (Variables|/Game/Blueprints/UI/Menus/BP_PauseMenuUI.BP_PauseMenuUI_C|GetPlayingAnimation _pausemenu)))
              (Widget|RemovefromParent _pausemenu)))
          (else
            (goto _label)))))))

(event Input|ActionEvents|InputActionMenuUp
  (params (Key :type Key%20Structure :default "None"))
  (bind _pausemenu (Variables|Default|GetPauseMenu))
  ;[1 1 1] MenuUpDown
  (:Pressed
    (if (Variables|Default|GetInSettings)
      (switch int (Variables|Default|GetSelectedTab)
        (:0
          (Default|SwitchVideoSelection _pausemenu))
        (:2
          (Default|SwitchControlsSelection _pausemenu)))
      (else
        (bind _newselectionnumber (CallFunction|SwitchSelectionNumber true 4 (Variables|Default|GetSelectedOption)))
        (Variables|Default|SetSelectedOption _newselectionnumber)
        (Default|SelectOption (Variables|Default|GetPauseMenu) (Variables|Default|GetSelectedOption))))))

(event Input|ActionEvents|InputActionMenuDown
  (params (Key :type Key%20Structure :default "None"))
  (bind _pausemenu (Variables|Default|GetPauseMenu))
  ;[1 1 1] MenuUpDown
  (:Pressed
    (if (Variables|Default|GetInSettings)
      (switch int (Variables|Default|GetSelectedTab)
        (:0
          (Default|SwitchVideoSelection _pausemenu))
        (:2
          (Default|SwitchControlsSelection _pausemenu)))
      (else
        (bind _newselectionnumber (CallFunction|SwitchSelectionNumber false 4 (Variables|Default|GetSelectedOption)))
        (Variables|Default|SetSelectedOption _newselectionnumber)
        (Default|SelectOption (Variables|Default|GetPauseMenu) (Variables|Default|GetSelectedOption))))))

(event Input|ActionEvents|InputActionMenuLeft
  (params (Key :type Key%20Structure :default "None"))
  (bind _pausemenu (Variables|Default|GetPauseMenu))
  ;[1 1 1] SettingsLeftRight
  (:Pressed
    (if (Variables|Default|GetInSettings)
      (switch int (Variables|Default|GetSelectedTab)
        (:1
          (Default|AdjustVolume _pausemenu -1))
        (:2
          (if (Variables|/Game/Blueprints/UI/Menus/BP_PauseMenuUI.BP_PauseMenuUI_C|GetInInputs _pausemenu)
            (Default|SwitchInputsSelection _pausemenu)
            (else
              (Default|SwitchAxisSelection _pausemenu))))))))

(event Input|ActionEvents|InputActionSwitchTabLeft
  (params (Key :type Key%20Structure :default "None"))
  ;[1 1 1] SwitchTab
  (:Pressed
    (if (Variables|Default|GetInSettings)
      (bind _newselectionnumber (CallFunction|SwitchSelectionNumber true 3 (Variables|Default|GetSelectedTab)))
      (Variables|Default|SetSelectedTab _newselectionnumber)
      (Default|SelectTab (Variables|Default|GetPauseMenu) (Variables|Default|GetSelectedTab) true))))

(event Input|ActionEvents|InputActionMenuRight
  (params (Key :type Key%20Structure :default "None"))
  (bind _pausemenu (Variables|Default|GetPauseMenu))
  ;[1 1 1] SettingsLeftRight
  (:Pressed
    (if (Variables|Default|GetInSettings)
      (switch int (Variables|Default|GetSelectedTab)
        (:1
          (Default|AdjustVolume _pausemenu 1))
        (:2
          (if (Variables|/Game/Blueprints/UI/Menus/BP_PauseMenuUI.BP_PauseMenuUI_C|GetInInputs _pausemenu)
            (Default|SwitchInputsSelection _pausemenu)
            (else
              (Default|SwitchAxisSelection _pausemenu))))))))

(event Input|ActionEvents|InputActionSwitchTabRight
  (params (Key :type Key%20Structure :default "None"))
  ;[1 1 1] SwitchTab
  (:Pressed
    (if (Variables|Default|GetInSettings)
      (bind _newselectionnumber (CallFunction|SwitchSelectionNumber false 3 (Variables|Default|GetSelectedTab)))
      (Variables|Default|SetSelectedTab _newselectionnumber)
      (Default|SelectTab (Variables|Default|GetPauseMenu) (Variables|Default|GetSelectedTab) false))))

(event Input|ActionEvents|InputActionMenuValidate
  (params (Key :type Key%20Structure :default "None"))
  (bind _pausemenu (Variables|Default|GetPauseMenu))
  (bind _gamemode (Variables|Default|GetGameMode))
  (bind _gamemode_2 (Variables|Default|GetGameMode))
  ;[1 1 1] MenuValidate
  (:Pressed
    (if (Variables|Default|GetInSettings)
      (if (and (== (Variables|Default|GetSelectedTab) 2) (not (Variables|/Game/Blueprints/UI/Menus/BP_PauseMenuUI.BP_PauseMenuUI_C|GetInInputs _pausemenu)))
        (if (Variables|/Game/Blueprints/UI/Menus/BP_PauseMenuUI.BP_PauseMenuUI_C|GetInYAxis _pausemenu)
          (Default|InvertCameraYAxis _gamemode)
          (else
            (Default|InvertCameraXAxis _gamemode))))
      (else
        (switch int (Variables|Default|GetSelectedOption)
          (:Default
            (CallFunction|ActivatePause :!label _label))
          (:0
            (goto _label))
          (:1
            (Utilities|FlowControl|Sequence
              (:then_0
                (goto _label))
              (:then_1
                (bind _returnvalue (Game|GetCurrentLevelName true))
                (Default|LoadLevel (Variables|Default|GetGameMode) (Utilities|String|StringToName _returnvalue)))))
          (:2
            (CallFunction|OpenSettings))
          (:3
            (Utilities|FlowControl|Sequence
              (:then_0
                (goto _label))
              (:then_1
                (Default|LoadLevel _gamemode_2 (Variables|/Game/Blueprints/GameManagement/BP_BimBallGameMode.BP_BimBallGameMode_C|GetHubLevel _gamemode_2))))))))))

(event Input|ActionEvents|InputActionMenuBack
  (params (Key :type Key%20Structure :default "None"))
  ;[1 1 1] MenuBack
  (:Pressed
    (if (Variables|Default|GetInSettings)
      (CallFunction|OpenSettings)
      (else
        (CallFunction|ActivatePause)))))

(fn ConstructionScript)

(fn SwitchSelectionNumber
  (params (Previous :type Boolean) (SelectionAmount :type Integer) (CurrentSelection :type Integer))
  (bind _returnvalue (Class|KismetSystemLibrary|MakeLiteralInteger))
  (bind _returnvalue_2 (Class|KismetSystemLibrary|MakeLiteralInteger SelectionAmount))
  (bind _returnvalue_3 (- _returnvalue_2 1))
  (if Previous
    (if (== CurrentSelection _returnvalue)
      (return _returnvalue_3)
      (else
        (bind _result (Math|Integer|DecrementInt CurrentSelection)
          (:%20%20
            (return _result)))))
    (elif (== CurrentSelection _returnvalue_3)
      (return _returnvalue)
      (else
        (bind _result_2 (Math|Integer|IncrementInt CurrentSelection)
          (:%20%20
            (return _result_2)))))))