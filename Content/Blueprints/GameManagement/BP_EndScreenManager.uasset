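; End screen manager for BimBall that announces the touchdown scorer, then shows a victory or defeat menu.
; On BeginPlay it disables player input, reuses the steal banner, and waits on a dilation-proof Timeline matched to that animation.
; It then pauses the game and repurposes BP_PauseMenuUI as the end menu.
; Up and Down share a FlipFlop between replay and quit, which load the current or hub level through the GameMode.
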(event EventTick
  (params (DeltaSeconds :type Float%20%28single-precision%29))
  ;[1 1 1] OnSpawn
)

(event EventBeginPlay
  (bind _timer (Variables|Default|GetTimer))
  ;[1 1 1] OnSpawn
  ;;[1 1 1] BeginPlay
  (Utilities|FlowControl|Sequence
    (:then_0
      (bind _asbp_bim_ball_character (Utilities|Casting|CastToBP_BimBallCharacter (Game|GetPlayerCharacter 0)))
      (bind _output_get (Variables|Default|SetPlayerEntity _asbp_bim_ball_character))
      (Input|DisableInput _asbp_bim_ball_character (Game|GetPlayerController 0))
      (bind _asbp_bim_ball_game_mode (Utilities|Casting|CastToBP_BimBallGameMode (Game|GetGameMode)))
      (bind _output_get_2 (Variables|Default|SetGameMode _asbp_bim_ball_game_mode)))
    (:then_1
      (Rendering|Components|TextRender|SetText (Variables|/Game/Blueprints/UI/InGame/Player/BP_PlayerUI.BP_PlayerUI_C|GetText1 (Variables|/Game/Blueprints/Entity/Player/BP_BimBallCharacter.BP_BimBallCharacter_C|GetPlayerUI (Variables|Default|GetPlayerEntity))) (select (== (Variables|/Game/Blueprints/GameManagement/BP_BimBallGameMode.BP_BimBallGameMode_C|GetWinningEntity (Variables|Default|GetGameMode)) (Variables|Default|GetPlayerEntity)) "pLAYER " "eNEMY"))
      (Rendering|Components|TextRender|SetText (Variables|/Game/Blueprints/UI/InGame/Player/BP_PlayerUI.BP_PlayerUI_C|GetText2 (Variables|/Game/Blueprints/Entity/Player/BP_BimBallCharacter.BP_BimBallCharacter_C|GetPlayerUI (Variables|Default|GetPlayerEntity))) "tOUCHDOWN")
      (Default|BallSteal (Variables|Default|GetPlayerEntity)))
    (:then_2
      (Class|TimelineComponent|SetIgnoreTimeDilation _timer true)
      (Components|Timeline|SetPlayRate _timer (/ (Components|Timeline|GetTimelineLength _timer) (Class|WidgetAnimation|GetEndTime (Variables|/Game/Blueprints/UI/InGame/Player/BP_PlayerUI.BP_PlayerUI_C|GetStealBannerApparition (Variables|/Game/Blueprints/Entity/Player/BP_BimBallCharacter.BP_BimBallCharacter_C|GetPlayerUI (Variables|Default|GetPlayerEntity))))))
      (Timeline|Timer PlayFromStart
        (:Finished
          (Game|SetGamePaused true)
          (bind _returnvalue (UserInterface|CreateWidget "/Game/Blueprints/UI/Menus/BP_PauseMenuUI.BP_PauseMenuUI_C"))
          (Variables|Default|SetEndScreen _returnvalue)
          (Utilities|Casting|CastToBP_BimBallCharacter (Variables|/Game/Blueprints/GameManagement/BP_BimBallGameMode.BP_BimBallGameMode_C|GetWinningEntity _output_get_2)
            (:then
              (Variables|Default|SetPlayerVictory true))
            (:CastFailed
              (Variables|Default|SetPlayerVictory false)))
          ;;[1 1 1] ScreenSetUp
          (Utilities|FlowControl|Sequence
            (:then_0
              (Appearance|SetColorandOpacity (Variables|/Game/Blueprints/UI/Menus/BP_PauseMenuUI.BP_PauseMenuUI_C|GetMenuTitle (Variables|Default|GetEndScreen)) (select (Variables|Default|GetPlayerVictory) (Utilities|Struct|MakeSlateColor "(R=0.000000,G=0.679543,B=0.219526,A=1.000000)") (Utilities|Struct|MakeSlateColor "(R=1.000000,G=0.057805,B=0.057805,A=1.000000)")) :!class /Script/UMG.TextBlock)
              (Rendering|Components|TextRender|SetText (Variables|/Game/Blueprints/UI/Menus/BP_PauseMenuUI.BP_PauseMenuUI_C|GetMenuTitle (Variables|Default|GetEndScreen)) (select (Variables|Default|GetPlayerVictory) "VICTORY" "DEFEAT"))
              (Rendering|Components|TextRender|SetText (Variables|/Game/Blueprints/UI/Menus/BP_PauseMenuUI.BP_PauseMenuUI_C|GetMenuOption2 (Variables|Default|GetEndScreen)) (select (Variables|Default|GetPlayerVictory) "Play Again" "Try Again"))
              (Rendering|Components|TextRender|SetText (Variables|/Game/Blueprints/UI/Menus/BP_PauseMenuUI.BP_PauseMenuUI_C|GetMenuOption3 (Variables|Default|GetEndScreen)) "Quit"))
            (:then_1
              (Widget|SetVisibility (Variables|/Game/Blueprints/UI/Menus/BP_PauseMenuUI.BP_PauseMenuUI_C|GetMenuOption1 (Variables|Default|GetEndScreen)) "Collapsed")
              (Widget|SetVisibility (Variables|/Game/Blueprints/UI/Menus/BP_PauseMenuUI.BP_PauseMenuUI_C|GetMenuOption4 (Variables|Default|GetEndScreen)) "Collapsed"))
            (:then_2
              (UserInterface|Viewport|AddtoViewport (Variables|Default|GetEndScreen) 0))
            (:then_3
              (Default|OpenPauseMenu (Variables|Default|GetEndScreen) "Forward" (Variables|Default|GetSelectedOption))
              (Utilities|FlowControl|Delay (Class|WidgetAnimation|GetEndTime (Variables|/Game/Blueprints/UI/Menus/BP_PauseMenuUI.BP_PauseMenuUI_C|GetOpenMenu (Variables|Default|GetEndScreen)))))
            (:then_4
              (Input|EnableInput (Game|GetPlayerController 0)))))))))

(event Input|ActionEvents|InputActionMenuValidate
  (params (Key :type Key%20Structure :default "None"))
  ;[1 1 1] Navigation
  ;;[1 1 1] PressButton
  (:Pressed
    (bind _returnvalue (Game|GetCurrentLevelName true))
    (Default|PressOption (Variables|Default|GetEndScreen))
    (Default|LoadLevel (Variables|Default|GetGameMode) (Utilities|Select :Index (Variables|Default|GetSelectedOption) :Option%200 "None" :Option%201 (Utilities|String|StringToName _returnvalue) :Option%202 (Variables|/Game/Blueprints/GameManagement/BP_BimBallGameMode.BP_BimBallGameMode_C|GetHubLevel (Variables|Default|GetGameMode)) :Option%203 "None"))))

(event Input|ActionEvents|InputActionMenuBack
  (params (Key :type Key%20Structure :default "None"))
  ;[1 1 1] Navigation
  ;;[1 1 1] PressButton
  (:Pressed
    (Default|LoadLevel (Variables|Default|GetGameMode) (Variables|/Game/Blueprints/GameManagement/BP_BimBallGameMode.BP_BimBallGameMode_C|GetHubLevel (Variables|Default|GetGameMode)))))

(event Input|ActionEvents|InputActionMenuDown
  (params (Key :type Key%20Structure :default "None"))
  ;[1 1 1] Navigation
  ;;[1 1 1] SelectButton
  (:Pressed
    (Utilities|FlowControl|FlipFlop
      (:A
        (bind _result (Math|Integer|IncrementInt (Variables|Default|GetSelectedOption))
          (:%20%20
            (Variables|Default|SetSelectedOption _result))))
      (:B
        (bind _result_2 (Math|Integer|DecrementInt (Variables|Default|GetSelectedOption))
          (:%20%20
            (Variables|Default|SetSelectedOption _result_2)))))
    (Default|SelectOption (Variables|Default|GetEndScreen) (Variables|Default|GetSelectedOption))))

(event Input|ActionEvents|InputActionMenuUp
  (params (Key :type Key%20Structure :default "None"))
  ;[1 1 1] Navigation
  ;;[1 1 1] SelectButton
  (:Pressed
    (Utilities|FlowControl|FlipFlop
      (:A
        (bind _result (Math|Integer|IncrementInt (Variables|Default|GetSelectedOption))
          (:%20%20
            (Variables|Default|SetSelectedOption _result))))
      (:B
        (bind _result_2 (Math|Integer|DecrementInt (Variables|Default|GetSelectedOption))
          (:%20%20
            (Variables|Default|SetSelectedOption _result_2)))))
    (Default|SelectOption (Variables|Default|GetEndScreen) (Variables|Default|GetSelectedOption))))

(fn ConstructionScript)