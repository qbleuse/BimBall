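; Main menu manager actor that runs BimBall's title menu: Play, Settings or Quit.
; On BeginPlay it disables player control and repurposes a pause menu widget as the settings screen.
; Menu input actions route by state flags to main menu, settings options or tabbed panel (video, volume, controls), with FlipFlops toggling open and close animations.
; Play re-enables the BimBall controller and character, then destroys the manager.
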(event Custom|SettingsDown
  (bind _pausemenu (Variables|Default|GetPauseMenu))
  ;[1 1 1] Settings
  ;;[1 1 1] SettingsUpDown
  (if (Variables|Default|GetInSettingsPanel)
    (switch int (Variables|Default|GetSettingsSelectedTab)
      (:0
        (Default|SwitchVideoSelection _pausemenu))
      (:2
        (Default|SwitchControlsSelection _pausemenu)))
    (else
      (Utilities|FlowControl|FlipFlop
        (:A
          (bind _result (Math|Integer|IncrementInt (Variables|Default|GetSettingsSelectedOption))
            (:%20%20
              (Variables|Default|SetSettingsSelectedOption _result))))
        (:B
          (bind _result_2 (Math|Integer|DecrementInt (Variables|Default|GetSettingsSelectedOption))
            (:%20%20
              (Variables|Default|SetSettingsSelectedOption _result_2)))))
      (Default|SelectOption (Variables|Default|GetPauseMenu) (Variables|Default|GetSettingsSelectedOption)))))

(event Custom|SettingsValidate
  (bind _pausemenu (Variables|Default|GetPauseMenu))
  (bind _mainmenu (Variables|Default|GetMainMenu))
  ;[1 1 1] Settings
  ;;[1 1 1] SettingsValidate
  (if (Variables|Default|GetInSettingsPanel)
    (if (and (== (Variables|Default|GetSettingsSelectedTab) 2) (not (Variables|/Game/Blueprints/UI/Menus/BP_PauseMenuUI.BP_PauseMenuUI_C|GetInInputs _pausemenu)))
      (if (Variables|/Game/Blueprints/UI/Menus/BP_PauseMenuUI.BP_PauseMenuUI_C|GetInYAxis _pausemenu)
        (Utilities|FlowControl|Sequence
          (:then_0
            (bind _asbp_bim_ball_game_mode (Utilities|Casting|CastToBP_BimBallGameMode (Game|GetGameMode) :!label _label)))
          (:then_1
            (Default|InvertCameraYAxis _asbp_bim_ball_game_mode)))
        (else
          (Utilities|FlowControl|Sequence
            (:then_0
              (goto _label))
            (:then_1
              (Default|InvertCameraXAxis _asbp_bim_ball_game_mode))))))
    (else
      (switch int (Variables|Default|GetSettingsSelectedOption)
        (:2
          (CallFunction|OpenSettingsPanel))
        (:3
          (CallFunction|OpenSettingsMenu)
          (UserInterface|Animation|PlayAnimation _mainmenu (Variables|/Game/Blueprints/UI/Menus/BP_MainMenuUI.BP_MainMenuUI_C|GetSettingsPress _mainmenu) 0.0 1 "Reverse" 5.0 false))))))

(event Custom|OpenSettingsMenu
  ;[1 1 1] Settings
  ;;[1 1 1] OpenSettingsMenu
  (bind _isa (Utilities|FlowControl|FlipFlop)
    (:A
      _)
    (:B
      _))
  (Default|OpenPauseMenu (Variables|Default|GetPauseMenu) (select _isa "Forward" "Reverse") (Variables|Default|GetSettingsSelectedOption) (Variables|Default|GetSettingsSelectedTab))
  (Variables|Default|SetInMainMenu (not _isa)))

(event Custom|OpenSettingsPanel
  ;[1 1 1] Settings
  ;;[1 1 1] OpenSettingsPanel
  (bind _isa (Utilities|FlowControl|FlipFlop)
    (:A
      _)
    (:B
      _))
  (Default|OpenSettingsPanel (Variables|Default|GetPauseMenu) (select _isa "Forward" "Reverse") false)
  (Variables|Default|SetInSettingsPanel _isa))

(event Custom|SettingsBack
  (bind _mainmenu (Variables|Default|GetMainMenu))
  ;[1 1 1] Settings
  ;;[1 1 1] SettingsBack
  (if (Variables|Default|GetInSettingsPanel)
    (CallFunction|OpenSettingsPanel)
    (else
      (CallFunction|OpenSettingsMenu)
      (UserInterface|Animation|PlayAnimation _mainmenu (Variables|/Game/Blueprints/UI/Menus/BP_MainMenuUI.BP_MainMenuUI_C|GetSettingsPress _mainmenu) 0.0 1 "Reverse" 5.0 false))))

(event Custom|PlayGame
  ;[1 1 1] PlayGame
  (bind _asbim_ball_controller (Utilities|Casting|CastToBimBallController (Game|GetPlayerController 0)))
  (Class|BimBallController|Enable _asbim_ball_controller)
  (Input|EnableInput (Game|GetPlayerCharacter 0) _asbim_ball_controller)
  (Actor|DestroyActor))

(event Custom|MenuSelectUp
  ;[1 1 1] Navigation
  ;;[1 1 1] SelectButton
  (if (== (Variables|Default|GetMenuSelectedButton) (Class|KismetSystemLibrary|MakeLiteralInteger))
    (Variables|Default|SetMenuSelectedButton (Class|KismetSystemLibrary|MakeLiteralInteger 2))
    (else
      (bind _result (Math|Integer|DecrementInt (Variables|Default|GetMenuSelectedButton))
        (:%20%20
          (Variables|Default|SetMenuSelectedButton _result)))))
  (Default|SelectMenuButton (Variables|Default|GetMainMenu) (Variables|Default|GetMenuSelectedButton)))

(event Custom|MenuSelectDown
  ;[1 1 1] Navigation
  ;;[1 1 1] SelectButton
  (if (== (Variables|Default|GetMenuSelectedButton) (Class|KismetSystemLibrary|MakeLiteralInteger 2))
    (Variables|Default|SetMenuSelectedButton (Class|KismetSystemLibrary|MakeLiteralInteger))
    (else
      (bind _result (Math|Integer|IncrementInt (Variables|Default|GetMenuSelectedButton))
        (:%20%20
          (Variables|Default|SetMenuSelectedButton _result)))))
  (Default|SelectMenuButton (Variables|Default|GetMainMenu) (Variables|Default|GetMenuSelectedButton)))

(event Custom|SettingsUp
  (bind _pausemenu (Variables|Default|GetPauseMenu))
  ;[1 1 1] Settings
  ;;[1 1 1] SettingsUpDown
  (if (Variables|Default|GetInSettingsPanel)
    (switch int (Variables|Default|GetSettingsSelectedTab)
      (:0
        (Default|SwitchVideoSelection _pausemenu))
      (:2
        (Default|SwitchControlsSelection _pausemenu)))
    (else
      (Utilities|FlowControl|FlipFlop
        (:A
          (bind _result (Math|Integer|IncrementInt (Variables|Default|GetSettingsSelectedOption))
            (:%20%20
              (Variables|Default|SetSettingsSelectedOption _result))))
        (:B
          (bind _result_2 (Math|Integer|DecrementInt (Variables|Default|GetSettingsSelectedOption))
            (:%20%20
              (Variables|Default|SetSettingsSelectedOption _result_2)))))
      (Default|SelectOption (Variables|Default|GetPauseMenu) (Variables|Default|GetSettingsSelectedOption)))))

(event EventBeginPlay
  (bind _returnvalue (Game|GetPlayerController 0))
  ;[1 1 1] BeginPlay
  (Utilities|FlowControl|Sequence
    (:then_0
      (bind _asbp_main_menu_ui (Utilities|Casting|CastToBP_MainMenuUI (UserInterface|GetUserWidgetObject (Variables|Default|GetMainMenuWidget))))
      (Variables|Default|SetMainMenu _asbp_main_menu_ui))
    (:then_1
      ;;[1 1 1] ActivateMenu
      (bind _asbim_ball_controller (Utilities|Casting|CastToBimBallController _returnvalue))
      (Class|BimBallController|Disable _asbim_ball_controller)
      (Input|DisableInput (Game|GetPlayerCharacter 0) _returnvalue)
      (Input|EnableInput _returnvalue)
      (Default|SelectMenuButton (Variables|Default|GetMainMenu) (Variables|Default|GetMenuSelectedButton)))
    (:then_2
      ;;[1 1 1] SettingsPanelInstantiation
      (Utilities|FlowControl|Sequence
        (:then_0
          ;;;[1 1 1] SpawnWidget
          (bind _returnvalue_2 (UserInterface|CreateWidget "/Game/Blueprints/UI/Menus/BP_PauseMenuUI.BP_PauseMenuUI_C"))
          (Variables|Default|SetPauseMenu _returnvalue_2))
        (:then_1
          ;;;[1 1 1] ShiftContent
          (Rendering|Components|TextRender|SetText (Variables|/Game/Blueprints/UI/Menus/BP_PauseMenuUI.BP_PauseMenuUI_C|GetMenuTitle (Variables|Default|GetPauseMenu)) "MENU")
          (Rendering|Components|TextRender|SetText (Variables|/Game/Blueprints/UI/Menus/BP_PauseMenuUI.BP_PauseMenuUI_C|GetMenuOption3 (Variables|Default|GetPauseMenu)) "Settings")
          (Rendering|Components|TextRender|SetText (Variables|/Game/Blueprints/UI/Menus/BP_PauseMenuUI.BP_PauseMenuUI_C|GetMenuOption4 (Variables|Default|GetPauseMenu)) "Back"))
        (:then_2
          (Widget|SetVisibility (Variables|/Game/Blueprints/UI/Menus/BP_PauseMenuUI.BP_PauseMenuUI_C|GetMenuOption1 (Variables|Default|GetPauseMenu)) "Collapsed")
          (Widget|SetVisibility (Variables|/Game/Blueprints/UI/Menus/BP_PauseMenuUI.BP_PauseMenuUI_C|GetMenuOption2 (Variables|Default|GetPauseMenu)) "Collapsed"))))))

(event Input|ActionEvents|InputActionMenuValidate
  (params (Key :type Key%20Structure :default "None"))
  (bind _returnvalue (Game|GetPlayerController 0))
  (bind _mainmenu (Variables|Default|GetMainMenu))
  ;[1 1 1] Navigation
  ;;[1 1 1] PressButton
  (:Pressed
    (if (Variables|Default|GetInMainMenu)
      (Default|PressMenuButton _mainmenu)
      (Input|DisableInput _returnvalue)
      (Utilities|FlowControl|Delay (/ (Class|WidgetAnimation|GetEndTime (Variables|/Game/Blueprints/UI/Menus/BP_MainMenuUI.BP_MainMenuUI_C|GetPlayingAnimation _mainmenu)) (Variables|/Game/Blueprints/UI/Menus/BP_MainMenuUI.BP_MainMenuUI_C|GetPlaybackSpeed _mainmenu)))
      (switch int (Variables|Default|GetMenuSelectedButton)
        (:0
          (CallFunction|PlayGame))
        (:1
          (Utilities|FlowControl|Sequence
            (:then_0
              (Utilities|FlowControl|DoOnce false
                (:Completed
                  (UserInterface|Viewport|AddtoViewport (Variables|Default|GetPauseMenu) 0))))
            (:then_1
              (CallFunction|OpenSettingsMenu)
              (CallFunction|OpenSettingsPanel)
              (Input|EnableInput _returnvalue))))
        (:2
          (Game|QuitGame 0 "Quit" false)))
      (else
        (CallFunction|SettingsValidate)))))

(event Input|ActionEvents|InputActionMenuBack
  (params (Key :type Key%20Structure :default "None"))
  ;[1 1 1] Navigation
  ;;[1 1 1] PressButton
  (:Pressed
    (if (not (Variables|Default|GetInMainMenu))
      (CallFunction|SettingsBack))))

(event Input|ActionEvents|InputActionMenuDown
  (params (Key :type Key%20Structure :default "None"))
  ;[1 1 1] Navigation
  ;;[1 1 1] SelectButton
  (:Pressed
    (if (Variables|Default|GetInMainMenu)
      (CallFunction|MenuSelectDown)
      (else
        (CallFunction|SettingsDown)))))

(event Input|ActionEvents|InputActionSwitchTabLeft
  (params (Key :type Key%20Structure :default "None"))
  ;[1 1 1] Settings
  ;;[1 1 1] SwitchTab
  (:Pressed
    (if (not (Variables|Default|GetInMainMenu))
      (bind _newselectionnumber (CallFunction|SwitchSelectionNumber true 3 (Variables|Default|GetSettingsSelectedTab)))
      (Variables|Default|SetSettingsSelectedTab _newselectionnumber) ; Hey
      (Default|SelectTab (Variables|Default|GetPauseMenu) (Variables|Default|GetSettingsSelectedTab) true))))

(event Input|ActionEvents|InputActionSwitchTabRight
  (params (Key :type Key%20Structure :default "None"))
  ;[1 1 1] Settings
  ;;[1 1 1] SwitchTab
  (:Pressed
    (if (not (Variables|Default|GetInMainMenu))
      (bind _newselectionnumber (CallFunction|SwitchSelectionNumber false 3 (Variables|Default|GetSettingsSelectedTab)))
      (Variables|Default|SetSettingsSelectedTab _newselectionnumber)
      (Default|SelectTab (Variables|Default|GetPauseMenu) (Variables|Default|GetSettingsSelectedTab) false))))

(event Input|ActionEvents|InputActionMenuLeft
  (params (Key :type Key%20Structure :default "None"))
  (bind _pausemenu (Variables|Default|GetPauseMenu))
  ;[1 1 1] Settings
  ;;[1 1 1] SettingsLeftRight
  (:Pressed
    (if (not (Variables|Default|GetInMainMenu))
      (switch int (Variables|Default|GetSettingsSelectedTab)
        (:1
          (Default|AdjustVolume _pausemenu -1))
        (:2
          (if (Variables|/Game/Blueprints/UI/Menus/BP_PauseMenuUI.BP_PauseMenuUI_C|GetInInputs _pausemenu)
            (Default|SwitchInputsSelection _pausemenu)
            (else
              (Default|SwitchAxisSelection _pausemenu))))))))

(event Input|ActionEvents|InputActionMenuRight
  (params (Key :type Key%20Structure :default "None"))
  (bind _pausemenu (Variables|Default|GetPauseMenu))
  ;[1 1 1] Settings
  ;;[1 1 1] SettingsLeftRight
  (:Pressed
    (if (not (Variables|Default|GetInMainMenu))
      (switch int (Variables|Default|GetSettingsSelectedTab)
        (:1
          (Default|AdjustVolume _pausemenu 1))
        (:2
          (if (Variables|/Game/Blueprints/UI/Menus/BP_PauseMenuUI.BP_PauseMenuUI_C|GetInInputs _pausemenu)
            (Default|SwitchInputsSelection _pausemenu)
            (else
              (Default|SwitchAxisSelection _pausemenu))))))))

(event Input|ActionEvents|InputActionMenuUp
  (params (Key :type Key%20Structure :default "None"))
  ;[1 1 1] Navigation
  ;;[1 1 1] SelectButton
  (:Pressed
    (if (Variables|Default|GetInMainMenu)
      (CallFunction|MenuSelectUp)
      (else
        (CallFunction|SettingsUp)))))

(fn ConstructionScript)

(fn SwitchSelectionNumber
  (params (Prev :type Boolean) (SelectAmount :type Integer) (CurrentSelect :type Integer))
  (bind _returnvalue (Class|KismetSystemLibrary|MakeLiteralInteger))
  (bind _returnvalue_2 (Class|KismetSystemLibrary|MakeLiteralInteger SelectAmount))
  (bind _returnvalue_3 (- _returnvalue_2 1))
  (if Prev
    (if (== CurrentSelect _returnvalue)
      (return _returnvalue_3)
      (else
        (bind _result (Math|Integer|DecrementInt CurrentSelect)
          (:%20%20
            (return _result)))))
    (elif (== CurrentSelect _returnvalue_3)
      (return _returnvalue)
      (else
        (bind _result_2 (Math|Integer|IncrementInt CurrentSelect)
          (:%20%20
            (return _result_2)))))))