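; BP_BimBallGameMode is the BimBall game mode, handling display settings, camera axis inversion, level loading and match end through custom events.
; Resolution changes also recompute the ball indicator's screen bounds on the player character, while inversion events toggle flags via FlipFlops.
; EndGame records the winner and spawns an end-screen manager; LoadLevel opens maps after a randomized delay.
; LevelTransition plays a duration-scaled fade widget; AdjustVolume is an empty stub.
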(event Custom|EndGame
  (params (ScoringEntity :type Object%20Object%20Reference))
  ;[1 1 1] EndGame
  (Variables|Default|SetWinningEntity ScoringEntity)
  (Game|SpawnActorfromClass "/Game/Blueprints/GameManagement/BP_EndScreenManager.BP_EndScreenManager_C" (Math|Transform|MakeTransform "0, 0, 0" "0, 0, 0" "1,1,1") "Undefined" 0 0))

(event Custom|InvertCameraYAxis
  ;[1 1 1] AxisInversion
  (bind _isa (Utilities|FlowControl|FlipFlop)
    (:A
      _)
    (:B
      _))
  (Variables|Default|SetCamYAxisInverted _isa))

(event Custom|InvertCameraXAxis
  ;[1 1 1] AxisInversion
  (bind _isa (Utilities|FlowControl|FlipFlop)
    (:A
      _)
    (:B
      _))
  (Variables|Default|SetCamXAxisInverted _isa))

(event Custom|ChangeResolution
  (params (Resolution :type Int%20Point%20Structure))
  ;[1 1 1] ChangeDisplay&Resolution
  (Utilities|FlowControl|Sequence
    (:then_0
      (bind _returnvalue (Settings|GetGameUserSettings)))
    (:then_1
      (Class|GameUserSettings|SetScreenResolution _returnvalue (Utilities|Struct|MakeIntPoint (.x Resolution) (.y Resolution)))
      (bind _output_get (Variables|Default|SetHalfScreenResolution (Math|Vector2D|MakeVector2D (Math|Conversions|ToFloat(Integer) (/ (.x Resolution) 2)) (Math|Conversions|ToFloat(Integer) (/ (.y Resolution) 2)))))
      (bind _asbp_bim_ball_character (Utilities|Casting|CastToBP_BimBallCharacter (Game|GetPlayerCharacter 0)))
      (Variables|/Game/Blueprints/Props/Ball/BP_Ball.BP_Ball_C|SetBallIndicatorBounds (Variables|/Game/Blueprints/Entity/Player/BP_BimBallCharacter.BP_BimBallCharacter_C|GetGiveBallReference _asbp_bim_ball_character) (- _output_get (Variables|/Game/Blueprints/Props/Ball/BP_Ball.BP_Ball_C|GetBallIndicatorOffset (Variables|/Game/Blueprints/Entity/Player/BP_BimBallCharacter.BP_BimBallCharacter_C|GetGiveBallReference _asbp_bim_ball_character)))))))

(event Custom|ChangeDisplayMode
  (params (Mode :type EWindowMode%20Enum :default "Fullscreen"))
  ;[1 1 1] ChangeDisplay&Resolution
  (Utilities|FlowControl|Sequence
    (:then_0
      (bind _returnvalue (Settings|GetGameUserSettings)))
    (:then_1
      (Class|GameUserSettings|SetFullscreenMode _returnvalue Mode))))

(event Custom|LoadLevel
  (params (Level :type Name))
  (bind _minimumloadingtime (Variables|Default|GetMinimumLoadingTime))
  (bind _loadingtimefluctuation (Variables|Default|GetLoadingTimeFluctuation))
  ;[1 1 1] LoadLevel
  (Game|SpawnActorfromClass "/Game/Blueprints/GameManagement/BP_LoadingScreen.BP_LoadingScreen_C" (Math|Transform|MakeTransform "0, 0, 0" "0, 0, 0" "1,1,1") "Undefined" 0 0)
  (Utilities|FlowControl|Delay (Math|Random|RandomFloatinRange (- _minimumloadingtime _loadingtimefluctuation) (+ _minimumloadingtime _loadingtimefluctuation)))
  (Game|OpenLevel(byName) Level))

(event Custom|LevelTransition
  (params (TransitionDuration :type Float%20%28single-precision%29))
  ;[1 1 1] LevelTransition
  (bind _asbp_bim_ball_character (Utilities|Casting|CastToBP_BimBallCharacter (Game|GetPlayerCharacter 0)))
  (bind _returnvalue (UserInterface|CreateWidget "/Game/Blueprints/UI/Menus/BP_TransitionScreen.BP_TransitionScreen_C"))
  (bind _output_get (Variables|Default|SetTransitionScreen _returnvalue))
  (UserInterface|Viewport|AddtoViewport _output_get 0)
  (UserInterface|Animation|PlayAnimation _output_get (Variables|/Game/Blueprints/UI/Menus/BP_TransitionScreen.BP_TransitionScreen_C|GetFadeAnimation _output_get) 0.0 1 "Forward" (/ (Class|WidgetAnimation|GetEndTime (Variables|/Game/Blueprints/UI/Menus/BP_TransitionScreen.BP_TransitionScreen_C|GetFadeAnimation _output_get)) TransitionDuration) false)
  (Utilities|FlowControl|Delay TransitionDuration)
  (Widget|RemovefromParent _output_get))

(event Custom|AdjustVolume
  (params (DesiredVolume :type Float%20%28single-precision%29)))

(event EventTick
  (params (DeltaSeconds :type Float%20%28single-precision%29)))

(fn ConstructionScript)