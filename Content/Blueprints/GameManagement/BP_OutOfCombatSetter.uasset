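; BP_OutOfCombatSetter is a zone actor that sets a BP_BimBallCharacter's engaged distance to zero while it overlaps, which by its name marks an out-of-combat area.
; Begin overlap on the CollisionComponent zeroes PlayerEngagedDist, and end overlap restores it from the character's EngagedDistance.
; A single InZone flag on the actor gates both events, so it tracks one occupant at a time rather than each character.
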(event OnComponentBeginOverlap(CollisionComponent)
  (params (OverlappedComponent :type Primitive%20Component%20Object%20Reference) (OtherActor :type Actor%20Object%20Reference) (OtherComp :type Primitive%20Component%20Object%20Reference) (OtherBodyIndex :type Integer) (bFromSweep :type Boolean) (SweepResult :type Hit%20Result%20Structure%20%28by%20ref%29))
  (bind _asbp_bim_ball_character (Utilities|Casting|CastToBP_BimBallCharacter OtherActor))
  (if (not (Variables|Default|GetInZone))
    (Variables|/Script/BimBall.BimBallCharacter|SetplayerEngagedDist _asbp_bim_ball_character 0.0)
    (Variables|Default|SetInZone true)))

(event OnComponentEndOverlap(CollisionComponent)
  (params (OverlappedComponent :type Primitive%20Component%20Object%20Reference) (OtherActor :type Actor%20Object%20Reference) (OtherComp :type Primitive%20Component%20Object%20Reference) (OtherBodyIndex :type Integer))
  (bind _asbp_bim_ball_character (Utilities|Casting|CastToBP_BimBallCharacter OtherActor))
  (if (Variables|Default|GetInZone)
    (Variables|/Script/BimBall.BimBallCharacter|SetplayerEngagedDist _asbp_bim_ball_character (Variables|/Game/Blueprints/Entity/Player/BP_BimBallCharacter.BP_BimBallCharacter_C|GetEngagedDistance _asbp_bim_ball_character))
    (Variables|Default|SetInZone false)))

(fn ConstructionScript)