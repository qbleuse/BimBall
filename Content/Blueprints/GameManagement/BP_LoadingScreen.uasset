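; BP_LoadingScreen is an actor that shows an animated loading screen when play begins.
; BeginPlay creates a BP_LoadingUI widget, adds it to the viewport and plays its OpenLoading animation at the widget's own playback speed.
; A looping timer on LoopDuration fires the Loading event, which appends a dot to the loading text and resets it to a single dot after three.
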(event Custom|Loading
  (bind _loadingscreen (Variables|Default|GetLoadingScreen))
  (bind _loadingtext (Variables|/Game/Blueprints/UI/Menus/BP_LoadingUI.BP_LoadingUI_C|GetLoadingText _loadingscreen))
  (bind _returnvalue (Class|TextBlock|GetText _loadingtext))
  (Rendering|Components|TextRender|SetText _loadingtext (select (Utilities|Enum|Equal(Enum) _returnvalue (Utilities|Text|ToText(String) "LOADING...")) (Utilities|Text|ToText(String) "LOADING.") (Utilities|Text|ToText(String) (Utilities|String|Append (Utilities|String|ToString(Text) _returnvalue) ".")))))

(event EventBeginPlay
  (bind _returnvalue (UserInterface|CreateWidget "/Game/Blueprints/UI/Menus/BP_LoadingUI.BP_LoadingUI_C"))
  (bind _output_get (Variables|Default|SetLoadingScreen _returnvalue))
  (UserInterface|Viewport|AddtoViewport _output_get 0)
  (UserInterface|Animation|PlayAnimation _output_get (Variables|/Game/Blueprints/UI/Menus/BP_LoadingUI.BP_LoadingUI_C|GetOpenLoading _output_get) 0.0 1 "Forward" (Variables|/Game/Blueprints/UI/Menus/BP_LoadingUI.BP_LoadingUI_C|GetPlaybackSpeed _output_get) false)
  (Utilities|Time|SetTimerbyEvent (delegate Custom|Loading) (Variables|Default|GetLoopDuration) true))

(event EventTick
  (params (DeltaSeconds :type Float%20%28single-precision%29)))

(fn ConstructionScript)