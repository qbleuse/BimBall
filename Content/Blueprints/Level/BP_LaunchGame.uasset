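; BP_LaunchGame is a level trigger that starts the game when the BimBall character walks into it.
; On BeginPlay it caches the BP_BimBallGameMode.
; When its collision component overlaps the character's capsule specifically, it calls the game mode's LoadLevel with the GameLevel stored on that game mode.
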(event OnComponentBeginOverlap(CollisionComponent)
  (params (OverlappedComponent :type Primitive%20Component%20Object%20Reference) (OtherActor :type Actor%20Object%20Reference) (OtherComp :type Primitive%20Component%20Object%20Reference) (OtherBodyIndex :type Integer) (bFromSweep :type Boolean) (SweepResult :type Hit%20Result%20Structure%20%28by%20ref%29))
  (bind _gamemode (Variables|Default|GetGameMode))
  (bind _asbp_bim_ball_character (Utilities|Casting|CastToBP_BimBallCharacter OtherActor))
  (if (== OtherComp (Variables|/Script/Engine.Character|GetCapsuleComponent _asbp_bim_ball_character))
    (Default|LoadLevel _gamemode (Variables|/Game/Blueprints/GameManagement/BP_BimBallGameMode.BP_BimBallGameMode_C|GetGameLevel _gamemode))))

(event EventBeginPlay
  (bind _asbp_bim_ball_game_mode (Utilities|Casting|CastToBP_BimBallGameMode (Game|GetGameMode)))
  (Variables|Default|SetGameMode _asbp_bim_ball_game_mode))

(fn ConstructionScript)