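; BP_Yard is a level section for the yard, where an enemy touchdown ends the game.
; It extends the parent's RunEnemyTouchdown, then passes the enemy to BP_BimBallGameMode's EndGame.
; From BeginPlay, a self-restarting timeline yaws the ZoneAura component, with play rate scaled so CylinderRotationRate sets each cycle's duration.
; StopRotation halts that timeline, and a leftover Lose call is never run.
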(event Custom|StopRotation
  (bind _materialrotation (Variables|Default|GetMaterialRotation))
  (bind _newtrack_0 (Timeline|MaterialRotation Stop)
    (:Update
      (Transformation|SetRelativeRotation (Variables|Default|GetZoneAura) (Math|Rotator|MakeRotator 0.0 0.0 _newtrack_0) false false))
    (:Finished
      (Components|Timeline|SetPlayRate _materialrotation (/ (Components|Timeline|GetTimelineLength _materialrotation) (Variables|Default|GetCylinderRotationRate)))
      (Timeline|MaterialRotation PlayFromStart))))

(event EventBeginPlay
  (bind _materialrotation (Variables|Default|GetMaterialRotation))
  (Components|Timeline|SetPlayRate _materialrotation (/ (Components|Timeline|GetTimelineLength _materialrotation) (Variables|Default|GetCylinderRotationRate)) :!label _label)
  (bind _newtrack_0 (Timeline|MaterialRotation PlayFromStart)
    (:Update
      (Transformation|SetRelativeRotation (Variables|Default|GetZoneAura) (Math|Rotator|MakeRotator 0.0 0.0 _newtrack_0) false false))
    (:Finished
      (goto _label))))

(event EventRunEnemyTouchdown
  (params (enemy :type Base%20Enemy%20Object%20Reference))
  (|CallParentFunction enemy)
  (bind _asbp_bim_ball_game_mode (Utilities|Casting|CastToBP_BimBallGameMode (Game|GetGameMode)))
  (Default|EndGame _asbp_bim_ball_game_mode enemy))

(fn ConstructionScript)