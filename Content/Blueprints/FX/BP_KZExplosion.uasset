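; BP_KZExplosion is a kamikaze explosion effect actor that plays its full sequence on BeginPlay, with sound, screenshake, controller rumble and a delayed screen-flash widget.
; One timeline drives both root scale and the "Tessellation Strength" material parameter to grow the blast.
; After a hold, the same timeline reverses at a decay rate, and a HasDecayed flag makes its second finish destroy the actor.
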(event EventBeginPlay
  (bind _vibrationduration (Variables|Default|GetVibrationDuration))
  (bind _explosiongrowth (Variables|Default|GetExplosionGrowth))
  (Utilities|FlowControl|Sequence
    (:then_0
      (bind _returnvalue (UserInterface|CreateWidget "/Game/Blueprints/FX/BP_FlashUI.BP_FlashUI_C"))
      (UserInterface|Viewport|AddtoViewport _returnvalue 0)
      (bind _asbp_bim_ball_character (Utilities|Casting|CastToBP_BimBallCharacter (Game|GetPlayerCharacter 0)))
      (Audio|PlaySoundatLocation "/Game/SFX/SoundWave_SFX/Kamikaze_Explosion_Fire.Kamikaze_Explosion_Fire" (Transformation|GetActorLocation) "0, 0, 0" 2.0 1.0 0.0 "/Game/SFX/Attenuation/GlobalAttenuation.GlobalAttenuation" 0 0)
      (Default|Screenshake _asbp_bim_ball_character 6e+01 _vibrationduration 0 0.05 0.0 0.0)
      (Game|Feedback|PlayDynamicForceFeedback (Game|GetPlayerController 0) (Variables|Default|GetVibrationIntensity) _vibrationduration true true true true)
      (Components|Timeline|SetPlayRate _explosiongrowth (/ (Components|Timeline|GetTimelineLength _explosiongrowth) (Variables|Default|GetExplosionGrowthDuration)))
      (bind _scale (Timeline|ExplosionGrowth PlayFromStart)
        (:Update
          (Transformation|SetRelativeScale3D (Variables|Default|GetDefaultSceneRoot) (Math|Vector|MakeVector (* _scale 11.0) (* _scale 11.0) (* _scale 11.0)))
          (Rendering|Material|SetScalarParameterValueonMaterials (Variables|Default|GetExplosionFX1) "Tessellation Strength" (+ 5e+01 (* _scale 1e+01))))
        (:Finished
          (if (Variables|Default|GetHasDecayed)
            (Actor|DestroyActor)
            (else
              (Utilities|FlowControl|Delay (Variables|Default|GetExplosionStayDuration))
              (Components|Timeline|SetPlayRate _explosiongrowth (/ 1.0 (Variables|Default|GetExplosionDecayDuration)))
              (Variables|Default|SetHasDecayed true)
              (Timeline|ExplosionGrowth ReverseFromEnd))))))
    (:then_1
      (Utilities|FlowControl|Delay 0.075)
      (Components|Animation|PlayAnimation _returnvalue (Variables|/Game/Blueprints/FX/BP_FlashUI.BP_FlashUI_C|GetScreenFlash _returnvalue) 0.0 1 "Forward" (Variables|/Game/Blueprints/FX/BP_FlashUI.BP_FlashUI_C|GetPlaybackSpeed _returnvalue)
        (:Finished
          (Widget|RemovefromParent _returnvalue))))))

(fn ConstructionScript)