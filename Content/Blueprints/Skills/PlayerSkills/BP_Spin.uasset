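; BP_Spin is a player skill for the Spin move of BP_BimBallCharacter.
; On Start it runs the parent logic, casts its owner to the character and calls SpinOnCD.
; If the character's SpinDealDamage flag is set, it overrides min and max damage with one fixed value.
; That value is BaseAttackDamage when CanEnhancedSpin is true, otherwise BaseSpinDamage.
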(event EventStart
  (bind _basespindamage (Variables|Default|GetBaseSpinDamage))
  (bind _baseattackdamage (Variables|Default|GetBaseAttackDamage))
  (|CallParentFunction)
  (bind _asbp_bim_ball_character (Utilities|Casting|CastToBP_BimBallCharacter (Variables|Default|Getowner)))
  (Default|SpinonCD _asbp_bim_ball_character)
  (if (Variables|/Game/Blueprints/Entity/Player/BP_BimBallCharacter.BP_BimBallCharacter_C|GetSpinDealDamage _asbp_bim_ball_character)
    (if (Variables|/Game/Blueprints/Entity/Player/BP_BimBallCharacter.BP_BimBallCharacter_C|GetCanEnhancedSpin _asbp_bim_ball_character)
      (Variables|Default|SetmaxDamages _baseattackdamage)
      (Variables|Default|SetminDamages _baseattackdamage)
      (else
        (Variables|Default|SetmaxDamages _basespindamage)
        (Variables|Default|SetminDamages _basespindamage)))))