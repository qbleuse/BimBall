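; BP_BallRush is a player skill Blueprint for the Ball Rush ability of BP_BimBallCharacter.
; On Start, it runs the parent logic, calls BallRushOnCD on the owning character and copies BallSnapRangeRadius into the BallRushRange of that character's ball reference.
; On End, it runs the parent logic and casts the owner, but the BallRushEnded call is disconnected and never runs.
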(event EventStart
  (|CallParentFunction)
  (bind _asbp_bim_ball_character (Utilities|Casting|CastToBP_BimBallCharacter (Variables|Default|Getowner)))
  (Default|BallRushonCD _asbp_bim_ball_character)
  (Variables|/Game/Blueprints/Props/Ball/BP_Ball.BP_Ball_C|SetBallRushRange (Variables|/Game/Blueprints/Entity/Player/BP_BimBallCharacter.BP_BimBallCharacter_C|GetGiveBallReference _asbp_bim_ball_character) (Variables|Default|GetballSnapRangeRadius)))

(event EventEnd
  (|CallParentFunction)
  (bind _asbp_bim_ball_character (Utilities|Casting|CastToBP_BimBallCharacter (Variables|Default|Getowner))))