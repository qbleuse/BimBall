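; Player basic attack combo skill for BP_BimBallCharacter, layering movement and hit feel on top of the parent skill's combo logic.
; Start and NextCombo run only when the character can attack away from NPCs, then share a path that sets attacking speed.
; With a valid aim target, it fires a randomized screenshake, slow-mo and enhanced spin window once until End resets it.
; NextCombo also triggers combo recovery at combo index 2.
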(event EventNextCombo
  (bind _asbp_bim_ball_character (Utilities|Casting|CastToBP_BimBallCharacter (Variables|Default|Getowner)))
  (bind _output_get (Variables|Default|SetOwnerCharacter _asbp_bim_ball_character))
  (if (and (Variables|/Game/Blueprints/Entity/Player/BP_BimBallCharacter.BP_BimBallCharacter_C|GetCanAttack _output_get) (not (Variables|/Game/Blueprints/Entity/Player/BP_BimBallCharacter.BP_BimBallCharacter_C|GetIsNearPNJ _output_get)))
    (|CallParentFunction)
    (if (== (Variables|Default|GetcomboIndex) 2)
      (Default|ComboRecovery (Variables|Default|GetOwnerCharacter)))
    (Utilities|FlowControl|Sequence
      (:then_0
        (Default|SetAttackingSpeed (Variables|Default|GetOwnerCharacter) false (Utilities|IsValid (Variables|Default|GetaimTarget))))
      (:then_1
        (if (and (Utilities|IsValid (Variables|Default|GetaimTarget)) (not (Variables|Default|GetIsAttacking)))
          (Default|Screenshake (Variables|Default|GetOwnerCharacter) (+ (Math|Random|RandomFloatinRange -2.5 2.5) (Variables|Default|GetScreenshakeIntensity)) (Variables|Default|GetScreenshakeDuration) 3 0.04 0.075 0.085)
          (Default|SlowMo (Variables|Default|GetOwnerCharacter) 0.05 0.05 0.035 0.225 0.08)
          (Variables|Default|SetIsAttacking true)
          (Default|EnhancedSpinWindow (Variables|Default|GetOwnerCharacter)))))))

(event EventStart
  (bind _asbp_bim_ball_character (Utilities|Casting|CastToBP_BimBallCharacter (Variables|Default|Getowner)))
  (bind _output_get (Variables|Default|SetOwnerCharacter _asbp_bim_ball_character))
  (if (and (Variables|/Game/Blueprints/Entity/Player/BP_BimBallCharacter.BP_BimBallCharacter_C|GetCanAttack _output_get) (not (Variables|/Game/Blueprints/Entity/Player/BP_BimBallCharacter.BP_BimBallCharacter_C|GetIsNearPNJ _output_get)))
    (|CallParentFunction)
    (Utilities|FlowControl|Sequence
      (:then_0
        (Default|SetAttackingSpeed (Variables|Default|GetOwnerCharacter) false (Utilities|IsValid (Variables|Default|GetaimTarget))))
      (:then_1
        (if (and (Utilities|IsValid (Variables|Default|GetaimTarget)) (not (Variables|Default|GetIsAttacking)))
          (Default|Screenshake (Variables|Default|GetOwnerCharacter) (+ (Math|Random|RandomFloatinRange -2.5 2.5) (Variables|Default|GetScreenshakeIntensity)) (Variables|Default|GetScreenshakeDuration) 3 0.04 0.075 0.085)
          (Default|SlowMo (Variables|Default|GetOwnerCharacter) 0.05 0.05 0.035 0.225 0.08)
          (Variables|Default|SetIsAttacking true)
          (Default|EnhancedSpinWindow (Variables|Default|GetOwnerCharacter)))))))

(event EventEnd
  ;[1 1 1] AttackingRunSpeed
  (|CallParentFunction)
  (Default|SetAttackingSpeed (Variables|Default|GetOwnerCharacter) true false)
  (Variables|Default|SetIsAttacking false))