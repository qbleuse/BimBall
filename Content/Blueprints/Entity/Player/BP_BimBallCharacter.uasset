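; Player character Blueprint for BimBall, layering feedback and ball-related hooks over its parent class.
; BeginPlay spawns the aim indicator, HUD and pause manager; Tick pins the indicator to the auto-aim target with controller rumble.
; Events handle hit flashes, ball-steal slow motion and chase speed, attack speed overrides, skill cooldown UI, and forwarding charge/aim states to the ball.
; Slow motion and most screenshakes use rate-scaled timelines that ignore time dilation.
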(event Custom|BallSteal
  (bind _returnvalue (Game|GetPlayerController 0))
  (bind _timer (Variables|Default|GetTimer))
  (bind _playerui (Variables|Default|GetPlayerUI))
  (bind _stealbannerapparitionbis (Variables|/Game/Blueprints/UI/InGame/Player/BP_PlayerUI.BP_PlayerUI_C|GetStealBannerApparitionBis _playerui))
  (bind _returnvalue_2 (Class|WidgetAnimation|GetEndTime _stealbannerapparitionbis))
  ;[1 1 1] BallSteal
  (Utilities|FlowControl|Sequence
    (:then_0
      (bind _asbim_ball_controller (Utilities|Casting|CastToBimBallController (Game|GetPlayerController 0)))
      (Class|BimBallController|Disable _asbim_ball_controller)
      (Input|DisableInput _returnvalue)
      (UserInterface|Animation|PlayAnimation _playerui _stealbannerapparitionbis 0.0 1 "Forward" 1.0 false)
      (CallFunction|SlowMo 0.5 0.2 _returnvalue_2 0.2 0.0)
      (Class|TimelineComponent|SetIgnoreTimeDilation _timer true)
      (Components|Timeline|SetPlayRate _timer (/ (Components|Timeline|GetTimelineLength _timer) _returnvalue_2))
      (Timeline|Timer PlayFromStart
        (:Finished
          (Input|EnableInput _returnvalue)
          (bind _asbim_ball_controller_2 (Utilities|Casting|CastToBimBallController (Game|GetPlayerController 0)))
          (Class|BimBallController|Enable _asbim_ball_controller_2))))
    (:then_1
      (bind _returnvalue_3 (UserInterface|CreateWidget "/Game/Blueprints/FX/BP_FlashUI.BP_FlashUI_C"))
      (UserInterface|Viewport|AddtoViewport _returnvalue_3 0)
      (Components|Animation|PlayAnimation _returnvalue_3 (Variables|/Game/Blueprints/FX/BP_FlashUI.BP_FlashUI_C|GetScreenFlash _returnvalue_3) 0.0 1 "Forward" (Variables|/Game/Blueprints/FX/BP_FlashUI.BP_FlashUI_C|GetPlaybackSpeed _returnvalue_3)
        (:Finished
          (Widget|RemovefromParent _returnvalue_3))))
    (:then_2
      (if (Variables|Default|GetUseCustomChaseSpeed)
        (CallFunction|SetCustomSpeed false (Variables|Default|GetChaseSpeed) 0.0)
        (Variables|Default|SetIsChasing true)))))

(event Custom|SlowMo
  (params (LerpDuration :type Float%20%28single-precision%29) (Amount :type Float%20%28single-precision%29) (AffectDuration :type Float%20%28single-precision%29) (LerpCurve :type Float%20%28single-precision%29) (StartupDelay :type Float%20%28single-precision%29))
  (bind _slowmotionduration (Variables|Default|GetSlowmotionDuration))
  (bind _slowmotionlerp (Variables|Default|GetSlowmotionLerp))
  ;[1 1 1] FX
  ;;[1 1 1] SlowMotion
  (Utilities|Time|SetGlobalTimeDilation 1.0)
  (Utilities|FlowControl|Delay StartupDelay)
  (if (!= LerpDuration 0.0)
    (Audio|Components|Audio|Stop _slowmotionlerp)
    (Class|TimelineComponent|SetIgnoreTimeDilation _slowmotionlerp true)
    (Components|Timeline|SetPlayRate _slowmotionlerp (/ (Components|Timeline|GetTimelineLength _slowmotionlerp) LerpDuration))
    (bind _lerpvalue (Timeline|SlowmotionLerp PlayFromStart)
      (:Update
        (if (!= LerpCurve 0.0)
          (if (> (Math|Float|Lerp (Class|GameplayStatics|GetGlobalTimeDilation) 0.0 _lerpvalue) Amount)
            (Utilities|Time|SetGlobalTimeDilation (Math|Float|Lerp (Class|GameplayStatics|GetGlobalTimeDilation) 0.0 _lerpvalue))
            (else
              (Utilities|Time|SetGlobalTimeDilation Amount :!label _label)))
          (elif (> _lerpvalue Amount)
            (Utilities|Time|SetGlobalTimeDilation _lerpvalue)
            (else
              (goto _label)))))
      (:Finished
        (Utilities|Time|SetGlobalTimeDilation Amount :!label _label_2)
        (Audio|Components|Audio|Stop _slowmotionduration)
        (Class|TimelineComponent|SetIgnoreTimeDilation _slowmotionduration true)
        (Components|Timeline|SetPlayRate _slowmotionduration (/ (Components|Timeline|GetTimelineLength _slowmotionduration) AffectDuration))
        (Timeline|SlowmotionDuration PlayFromStart
          (:Finished
            (Utilities|Time|SetGlobalTimeDilation 1.0)))))
    (else
      (goto _label_2))))

(event Custom|BallRushOnCD
  (bind _returnvalue (Class|KismetSystemLibrary|MakeLiteralInteger 1))
  (bind _returnvalue_2 (Math|Float|MakeLiteralFloat 0.4))
  (bind _playerui (Variables|Default|GetPlayerUI))
  ;[1 1 1] UICooldowns
  (Variables|Default|SetBallRushCD true)
  (Default|SkillonCD _playerui _returnvalue false)
  (Utilities|FlowControl|Delay _returnvalue_2)
  (Utilities|FlowControl|Delay (- (.cooldown (Variables|Default|GetballRushSub)) _returnvalue_2))
  (Variables|Default|SetBallRushCD false)
  (Default|SkillNotonCD _playerui _returnvalue false))

(event Custom|SpinEnded
  ;[1 1 1] UICooldowns
  (Utilities|FlowControl|Delay (- (.cooldown (Variables|Default|GetspinSub)) (Math|Float|MakeLiteralFloat 0.4)))
  (Variables|Default|SetSpinCD false)
  (Default|SkillNotonCD (Variables|Default|GetPlayerUI) (Class|KismetSystemLibrary|MakeLiteralInteger) false))

(event Custom|BallRushEnded
  ;[1 1 1] UICooldowns
  (Utilities|FlowControl|Delay (- (.cooldown (Variables|Default|GetballRushSub)) (Math|Float|MakeLiteralFloat 0.4)))
  (Variables|Default|SetBallRushCD false)
  (Default|SkillNotonCD (Variables|Default|GetPlayerUI) (Class|KismetSystemLibrary|MakeLiteralInteger 1) false))

(event Custom|Screenshake
  (params (Intensity :type Float%20%28single-precision%29) (MultipleShakesDuration :type Float%20%28single-precision%29) (ShakeType :type Integer) (LerpDuration :type Float%20%28single-precision%29) (RepositionmentDelay :type Float%20%28single-precision%29) (StartupDelay :type Float%20%28single-precision%29))
  (bind _returnvalue (Math|Random|RandomFloat))
  (bind _returnvalue_2 (Math|Random|RandomFloat))
  (bind _returnvalue_3 (Math|Random|RandomFloat))
  (bind _returnvalue_4 (Math|Random|RandomFloat))
  (bind _followcamera (Variables|Default|GetFollowCamera))
  (bind _screenshakes (Variables|Default|GetScreenshakes))
  (bind _followcamera_2 (Variables|Default|GetFollowCamera))
  (bind _screenshakelerping (Variables|Default|GetScreenshakeLerping))
  (bind _gamemode (Variables|Default|GetGameMode))
  (bind _followcamera_3 (Variables|Default|GetFollowCamera))
  (bind _returnvalue_5 (Math|Vector2D|MakeVector2D _returnvalue_2 _returnvalue))
  (bind _returnvalue_6 (Math|Vector2D|MakeVector2D _returnvalue_3 _returnvalue_4))
  (bind _halfscreenresolution (Variables|/Game/Blueprints/GameManagement/BP_BimBallGameMode.BP_BimBallGameMode_C|GetHalfScreenResolution _gamemode))
  (bind _returnvalue_7 (Math|Vector2D|Normalize2D _returnvalue_5))
  (bind _returnvalue_8 (Math|Vector2D|Normalize2D _returnvalue_6))
  ;[1 1 1] FX
  ;;[1 1 1] Screenshake(s)
  (Utilities|FlowControl|Delay StartupDelay)
  (switch int ShakeType
    (:Default
      ;;;[1 1 1] MultipleShakes
      (Class|TimelineComponent|SetIgnoreTimeDilation _screenshakes true :!label _label)
      (Audio|Components|Audio|Stop _screenshakes)
      (Components|Timeline|SetPlayRate _screenshakes (/ (Components|Timeline|GetTimelineLength _screenshakes) MultipleShakesDuration))
      (Timeline|Screenshakes PlayFromStart
        (:Update
          (Transformation|SetRelativeLocation _followcamera (* (Math|Vector|MakeVector 0.0 (.x _returnvalue_7) (.y _returnvalue_7)) Intensity) false false))
        (:Finished
          (Transformation|SetRelativeLocation _followcamera "0, 0, 0" false false))))
    (:0
      (goto _label))
    (:1
      ;;;[1 1 1] SingleShake
      (Transformation|SetRelativeLocation _followcamera_2 (* (Math|Vector|MakeVector 0.0 (.x _returnvalue_8) (.y _returnvalue_8)) Intensity) false false)
      (Utilities|FlowControl|Delay RepositionmentDelay)
      (Transformation|SetRelativeLocation _followcamera_2 "0, 0, 0" false false))
    (:2
      ;;;[1 1 1] CornerShake
      (Audio|Components|Audio|Stop (Variables|Default|GetScreenshakes))
      (Audio|Components|Audio|Stop _screenshakelerping)
      (Components|Timeline|SetPlayRate _screenshakelerping (/ (Components|Timeline|GetTimelineLength _screenshakelerping) LerpDuration))
      (Class|TimelineComponent|SetIgnoreTimeDilation _screenshakelerping true)
      (Variables|Default|SetCornerShakeVector (* (Math|Vector2D|Normalize2D (Math|Vector2D|MakeVector2D (* (.x _halfscreenresolution) (select (Math|Random|RandomBool) 1.0 -1.0)) (* (.y _halfscreenresolution) (select (Math|Random|RandomBool) 1.0 -1.0)))) Intensity))
      (bind _values (Timeline|ScreenshakeLerping PlayFromStart)
        (:Update
          (Transformation|SetRelativeLocation _followcamera_2 (Math|Vector|MakeVector 0.0 (.x (* (Variables|Default|GetCornerShakeVector) _values)) (.y (* (Variables|Default|GetCornerShakeVector) _values))) false false))
        (:Finished
          (Utilities|FlowControl|Delay RepositionmentDelay)
          (Transformation|SetRelativeLocation _followcamera_2 "0, 0, 0" false false))))
    (:3
      (Transformation|SetRelativeLocation _followcamera_3 (Math|Vector|MakeVector (* Intensity 7.0) 0.0 0.0) false false)
      (Utilities|FlowControl|RetriggerableDelay RepositionmentDelay)
      (Transformation|SetRelativeLocation _followcamera_3 (Math|Vector|MakeVector 0.0 0.0 0.0) false false))))

(event Custom|ComboRecovery
  ;[1 1 1] ComboRecovery
  (Variables|Default|SetCanAttack false)
  (Utilities|FlowControl|Delay (Variables|Default|GetComboRecoveryDuration))
  (Variables|Default|SetCanAttack true))

(event Custom|SetAttackingSpeed
  (params (Reset :type Boolean) (HasTarget :type Boolean))
  (bind _returnvalue (select HasTarget 1.0 2.0))
  (bind _attackwalkspeed (Variables|Default|GetAttackWalkSpeed))
  (bind _returnvalue_2 (* _attackwalkspeed _returnvalue))
  ;[1 1 1] SetAttackingSpeed
  (if Reset
    (Variables|Default|SetfightingSpeed (Variables|Default|GetBaseFightSpeed))
    (Variables|Default|SetrunSpeed (Variables|Default|GetBaseRunSpeed))
    (else
      (Variables|Default|SetfightingSpeed _returnvalue_2)
      (Variables|Default|SetrunSpeed _returnvalue_2)))
  (Utilities|FlowControl|RetriggerableDelay 0.2)
  (Variables|Default|SetfightingSpeed (Variables|Default|GetBaseFightSpeed))
  (Variables|Default|SetrunSpeed (Variables|Default|GetBaseRunSpeed)))

(event Custom|ComboBuffer
  (Class|BimBallCharacter|BasicAttack))

(event Custom|ControllerVibrations
  (params (Stop :type Boolean) (Intensity :type Float%20%28single-precision%29) (Duration :type Float%20%28single-precision%29))
  ;[1 1 1] FX
  ;;[1 1 1] ControllerVibrations
  (if Stop
    (goto _label Stop)
    (else
      (Game|Feedback|PlayDynamicForceFeedback (Game|GetPlayerController 0) Intensity Duration true true true true :!label _label))))

(event Custom|GiveBallRef
  (params (BallRef :type BP%20Ball%20Object%20Reference))
  ;[1 1 1] Make BP_Ball Ref accessible to anything..................
  (Variables|Default|SetGiveBallReference BallRef))

(event Custom|EnhancedSpinWindow
  ;[1 1 1] DamagingSpin
  (if (Variables|Default|GetSpinDealDamage)
    (Variables|Default|SetCanEnhancedSpin true)
    (Utilities|FlowControl|RetriggerableDelay (Variables|Default|GetEnhancedSpinTimer))
    (Variables|Default|SetCanEnhancedSpin false)))

(event Custom|SetCustomSpeed
  (params (Reset :type Boolean) (CustomSpeed :type Float%20%28single-precision%29) (Duration :type Float%20%28single-precision%29))
  ;[1 1 1] SetCustomSpeed
  (if Reset
    (Variables|Default|SetfightingSpeed (Variables|Default|GetBaseFightSpeed) :!label _label)
    (Variables|Default|SetrunSpeed (Variables|Default|GetBaseRunSpeed))
    (else
      (Variables|Default|SetfightingSpeed CustomSpeed)
      (Variables|Default|SetrunSpeed CustomSpeed)
      (if (!= Duration 0.0)
        (Utilities|FlowControl|Delay Duration)
        (goto _label)))))

(event Custom|SpinOnCD
  (bind _returnvalue (Class|KismetSystemLibrary|MakeLiteralInteger))
  (bind _returnvalue_2 (Math|Float|MakeLiteralFloat 0.4))
  (bind _playerui (Variables|Default|GetPlayerUI))
  ;[1 1 1] UICooldowns
  (Variables|Default|SetSpinCD true)
  (Default|SkillonCD _playerui _returnvalue false)
  (Utilities|FlowControl|Delay _returnvalue_2)
  (Utilities|FlowControl|Delay (- (.cooldown (Variables|Default|GetspinSub)) _returnvalue_2))
  (Variables|Default|SetSpinCD false)
  (Default|SkillNotonCD _playerui _returnvalue false))

(event EventDealDamages
  (params (attacker :type Actor%20Object%20Reference) (rawDamages :type Float%20%28single-precision%29))
  (bind _playerui (Variables|Default|GetPlayerUI))
  (bind _playerdamagesounds (Variables|Default|GetPlayerDamageSounds))
  ;[1 1 1] ReceiveDamage
  (|CallParentFunction attacker rawDamages)
  (if (> rawDamages 0.1)
    (bind _returnvalue (UserInterface|CreateWidget "/Game/Blueprints/FX/BP_FlashUI.BP_FlashUI_C"))
    (UserInterface|Viewport|AddtoViewport _returnvalue 0)
    (Variables|/Game/Blueprints/FX/BP_FlashUI.BP_FlashUI_C|SetFlashColor _returnvalue "(R=0.755208,G=0.019663,B=0.000000,A=1.000000)")
    (Widget|SetRenderOpacity _returnvalue 0.25)
    (UserInterface|Animation|PlayAnimation _playerui (Variables|/Game/Blueprints/UI/InGame/Player/BP_PlayerUI.BP_PlayerUI_C|GetReceiveHit _playerui) 0.0 1 "Forward" (Variables|/Game/Blueprints/UI/InGame/Player/BP_PlayerUI.BP_PlayerUI_C|GetPlaybackSpeed _playerui) false)
    (Utilities|Array|Shuffle _playerdamagesounds)
    (Audio|PlaySoundatLocation (Utilities|Array|Get(acopy) _playerdamagesounds (Math|Random|RandomIntegerinRange 0 (Utilities|Array|Length _playerdamagesounds))) (Transformation|GetActorLocation) "0, 0, 0" 0.6 1.0 0.0 0 0 0)
    (Components|Animation|PlayAnimation _returnvalue (Variables|/Game/Blueprints/FX/BP_FlashUI.BP_FlashUI_C|GetScreenFlash _returnvalue) 0.0 1 "Forward" (Variables|/Game/Blueprints/FX/BP_FlashUI.BP_FlashUI_C|GetPlaybackSpeed _returnvalue)
      (:Finished
        (Widget|RemovefromParent _returnvalue)))))

(event EventOnBallCharged
  (|CallParentFunction)
  (bind _asbp_ball (Utilities|Casting|CastToBP_Ball (Class|Entity|GetBall)))
  (Default|OnCharged _asbp_ball))

(event EventBeginPlay
  ;[1 1 1] BeginPlay
  ;;[1 1 1] Draw Widgets (keeping both for now because the 2nd one is still in work)
  (|CallParentFunction)
  (Utilities|FlowControl|Sequence
    (:then_0
      ;;[1 1 1] SpawnAimTargetIndicator
      (bind _returnvalue (Game|SpawnActorfromClass "/Game/Blueprints/UI/InGame/Enemy/BP_AimTarget.BP_AimTarget_C" (Math|Transform|MakeTransform "0, 0, 0") "Undefined" 0 0))
      (Variables|Default|SetAimTargetIndicator _returnvalue))
    (:then_1
      (bind _returnvalue_2 (UserInterface|CreateWidget "/Game/Blueprints/UI/InGame/Player/BP_PlayerUI.BP_PlayerUI_C"))
      (bind _output_get (Variables|Default|SetPlayerUI _returnvalue_2))
      (UserInterface|Viewport|AddtoViewport _output_get 0))
    (:then_2
      (bind _returnvalue_3 (Game|SpawnActorfromClass "/Game/Blueprints/GameManagement/BP_PauseManager.BP_PauseManager_C" (Math|Transform|MakeTransform "0, 0, 0") "Undefined" 0 0))
      (Variables|Default|SetPauseManager _returnvalue_3))
    (:then_3
      (Variables|Default|SetBaseRunSpeed (Variables|Default|GetrunSpeed))
      (Variables|Default|SetBaseFightSpeed (Variables|Default|GetfightingSpeed))
      (Variables|Default|SetEngagedDistance (Variables|Default|GetplayerEngagedDist)))
    (:then_4
      (bind _asbp_bim_ball_game_mode (Utilities|Casting|CastToBP_BimBallGameMode (Game|GetGameMode)))
      (Variables|Default|SetGameMode _asbp_bim_ball_game_mode))))

(event EventTick
  (params (DeltaSeconds :type Float%20%28single-precision%29))
  (bind _aimtargetindicator (Variables|Default|GetAimTargetIndicator))
  ;[1 1 1] Tick
  (|CallParentFunction DeltaSeconds)
  ;;[1 1 1] PlayerAiming
  (if (Variables|Default|GetisAiming)
    (if (!= (Transformation|GetDistanceTo (Class|BimBallCharacter|GetBallAutoAimTarget)) 0.0)
      (Transformation|AttachActorToActor _aimtargetindicator (Class|BimBallCharacter|GetBallAutoAimTarget) "Mesh" "SnapToTarget" "KeepRelative" "KeepWorld" true)
      (Transformation|SetActorRelativeLocation _aimtargetindicator (Math|Vector|MakeVector 0.0 0.0 (Variables|Default|GetEnemyHeight)))
      (Rendering|SetActorHiddenInGame _aimtargetindicator false)
      (Game|Feedback|PlayDynamicForceFeedback (Game|GetPlayerController 0) (/ (Variables|Default|GetcurrentBallChargeDuration) 2.0) -1.0 true true true true :!label _label)
      (else
        (Utilities|FlowControl|Sequence
          (:then_0
            (goto _label))
          (:then_1
            (Rendering|SetActorHiddenInGame _aimtargetindicator true :!label _label_2)))))
    (else
      (Utilities|FlowControl|Sequence
        (:then_0
          (goto _label Stop))
        (:then_1
          (goto _label_2))))))

(event EventOnJumped
  (bind _returnvalue (Transformation|GetActorLocation))
  ;[1 1 1] FX
  (Utilities|FlowControl|FlipFlop
    (:A
      (Audio|PlaySoundatLocation "/Game/SFX/SoundWave_SFX/Jump01.Jump01" _returnvalue "0, 0, 0" 1.0 1.0 0.0 "/Game/SFX/Attenuation/GlobalAttenuation.GlobalAttenuation" 0 0))
    (:B
      (Audio|PlaySoundatLocation "/Game/SFX/SoundWave_SFX/Jump02.Jump02" _returnvalue "0, 0, 0" 1.0 1.0 0.0 "/Game/SFX/Attenuation/GlobalAttenuation.GlobalAttenuation" 0 0))))

(event EventOnBallUncharged
  (|CallParentFunction)
  (bind _asbp_ball (Utilities|Casting|CastToBP_Ball (Class|Entity|GetBall)))
  (Default|OnUncharged _asbp_ball))

(event EventBall
  (params (b :type Ball%20Object%20Reference))
  ;[1 1 1] BallSteal
  ;;[1 1 1] RecoverBall
  (|CallParentFunction b)
  (if (Variables|Default|GetIsChasing)
    (Variables|Default|SetIsChasing false)
    (CallFunction|SetCustomSpeed true 0.0 0.0)))

(event EventOnAimStart
  (|CallParentFunction)
  (bind _asbp_ball (Utilities|Casting|CastToBP_Ball (Class|Entity|GetBall)))
  (Default|OnAimStart _asbp_ball))

(event EventOnAimEnd
  (|CallParentFunction)
  (bind _asbp_ball (Utilities|Casting|CastToBP_Ball (Class|Entity|GetBall)))
  (Default|OnAimEnd _asbp_ball))

(event Input|ActionEvents|InputActionQuit
  (params (Key :type Key%20Structure :default "None"))
  ;[1 1 1] ActivatePause
  (:Pressed
    (Default|ActivatePause (Variables|Default|GetPauseManager))))

(fn ConstructionScript)