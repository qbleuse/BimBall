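; Trainer NPC that shows a dialogue to the player when they come within its interaction range.
; On begin play it hands itself and the dialogue count to its widget-component dialogue UI, which yaws toward the camera every tick.
; Range overlaps toggle the character's near-NPC flag and custom speed, enable or disable input, and open or end dialogue.
; While input is enabled, validate opens or advances dialogue and back closes it.
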(event OnComponentBeginOverlap(InteractibleRange)
  (params (OverlappedComponent :type Primitive%20Component%20Object%20Reference) (OtherActor :type Actor%20Object%20Reference) (OtherComp :type Primitive%20Component%20Object%20Reference) (OtherBodyIndex :type Integer) (bFromSweep :type Boolean) (SweepResult :type Hit%20Result%20Structure%20%28by%20ref%29))
  ;[1 1 1] Overlap
  (bind _asbp_bim_ball_character (Utilities|Casting|CastToBP_BimBallCharacter OtherActor))
  (if (not (Variables|/Game/Blueprints/Entity/Player/BP_BimBallCharacter.BP_BimBallCharacter_C|GetIsNearPNJ _asbp_bim_ball_character))
    (Variables|/Game/Blueprints/Entity/Player/BP_BimBallCharacter.BP_BimBallCharacter_C|SetIsNearPNJ _asbp_bim_ball_character true)
    (Default|SetCustomSpeed _asbp_bim_ball_character false (Math|Float|MakeLiteralFloat 7e+02) 0.0)
    (Input|EnableInput (Game|GetPlayerController 0))
    (Default|OpenDialogue (Variables|Default|GetDialogueUI))))

(event OnComponentEndOverlap(InteractibleRange)
  (params (OverlappedComponent :type Primitive%20Component%20Object%20Reference) (OtherActor :type Actor%20Object%20Reference) (OtherComp :type Primitive%20Component%20Object%20Reference) (OtherBodyIndex :type Integer))
  ;[1 1 1] Overlap
  (bind _asbp_bim_ball_character (Utilities|Casting|CastToBP_BimBallCharacter OtherActor))
  (if (Variables|/Game/Blueprints/Entity/Player/BP_BimBallCharacter.BP_BimBallCharacter_C|GetIsNearPNJ _asbp_bim_ball_character)
    (Variables|/Game/Blueprints/Entity/Player/BP_BimBallCharacter.BP_BimBallCharacter_C|SetIsNearPNJ _asbp_bim_ball_character false)
    (Default|SetCustomSpeed _asbp_bim_ball_character true (Math|Float|MakeLiteralFloat 7e+02) 0.0)
    (Input|DisableInput (Game|GetPlayerController 0))
    (Default|EndDialogue (Variables|Default|GetDialogueUI))))

(event Custom|ActivatePNJ)

(event EventTick
  (params (DeltaSeconds :type Float%20%28single-precision%29))
  ;[1 1 1] Tick
  (Transformation|SetWorldRotation (Variables|Default|GetInteractionUI) (Math|Rotator|MakeRotator 0.0 0.0 (.yaw (Math|Rotator|FindLookatRotation (Transformation|GetActorLocation) (Camera|GetCameraLocation (Game|GetPlayerCameraManager 0))))) false false))

(event EventBeginPlay
  ;[1 1 1] Parenting
  (Utilities|FlowControl|Sequence
    (:then_0
      (bind _asbp_bim_ball_character (Utilities|Casting|CastToBP_BimBallCharacter (Game|GetPlayerCharacter 0)))
      (Variables|Default|SetPlayerEntity _asbp_bim_ball_character)
      (bind _asbp_dialogue_ui (Utilities|Casting|CastToBP_DialogueUI (UserInterface|GetUserWidgetObject (Variables|Default|GetInteractionUI))))
      (Variables|Default|SetDialogueUI _asbp_dialogue_ui)
      (Default|GetOwner _asbp_dialogue_ui self (Variables|Default|GetTotalDialogueAmount)))
    (:then_1
      (Variables|/Game/Blueprints/UI/InGame/HUB/PNJ/BP_DialogueUI.BP_DialogueUI_C|SetVisibilityMaxDistance (Variables|Default|GetDialogueUI) (Variables|Default|GetDialogueMaxDistance)))))

(event Input|ActionEvents|InputActionMenuValidate
  (params (Key :type Key%20Structure :default "None"))
  (bind _dialogueui (Variables|Default|GetDialogueUI))
  ;[1 1 1] Dialogue
  (:Pressed
    (if (== (Variables|/Game/Blueprints/UI/InGame/HUB/PNJ/BP_DialogueUI.BP_DialogueUI_C|GetDIalogueIndex _dialogueui) 0)
      (Default|OpenDialogue _dialogueui)
      (else
        (Default|NextDialogue _dialogueui "Forward")))))

(event Input|ActionEvents|InputActionMenuBack
  (params (Key :type Key%20Structure :default "None"))
  ;[1 1 1] Dialogue
  (:Pressed
    (Default|EndDialogue (Variables|Default|GetDialogueUI))))

(fn ConstructionScript)