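; Base enemy Blueprint that layers visual, audio and haptic feedback onto parent combat events, with a random soldier or elite mesh.
; Vulnerability toggles a material fresnel and a timeline-scaled AOE indicator.
; Attack events drive the EnemyUI reaction sprite and recolor the range indicator, while hits trigger impact particles, sounds or rumble, with ball hits adding screenshake and slow-mo.
; Ball events trigger the player's BallSteal unless enemies already stole it.
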(event EventBeginPlay
  ;[1 1 1] BeginPlay
  (|CallParentFunction)
  (bind _asbp_enemy_ui (Utilities|Casting|CastToBP_EnemyUI (Variables|/Script/Engine.ChildActorComponent|GetChildActor (Variables|Default|GetUI))))
  (Variables|Default|SetEnemyUI _asbp_enemy_ui)
  (Class|SkinnedMeshComponent|SetSkeletalMesh (Variables|Character|GetMesh) (Utilities|Select :Index (Math|Random|RandomIntegerinRange 0 1) :Option%200 "/Game/Meshes/ModularRPGHeroesPolyart/OneMeshCharacters/SoldierSK.SoldierSK" :Option%201 "/Game/Meshes/ModularRPGHeroesPolyart/OneMeshCharacters/SK_Elite.SK_Elite") false)
  (Class|BaseEnemy|ResetVulnerable))

(event EventOnHpZero
  (params (killer :type Actor%20Object%20Reference))
  ;[1 1 1] DeathFX
  (|CallParentFunction killer)
  (Utilities|FlowControl|Sequence
    (:then_0
      (CallFunction|AttackedCallback 2.8 3.0))
    (:then_1
      (Components|DestroyComponent (Variables|Default|GetUI))
      (Components|DestroyComponent (Variables|Default|GetVulnerableAOE))
      (Components|DestroyComponent (Variables|Default|GetAttackRange)))))

(event EventAttack
  (params (playerChar_ :type Bim%20Ball%20Character%20Object%20Reference))
  ;[1 1 1] AttackSprite
  (|CallParentFunction playerChar_)
  (Default|SetReaction :self (Variables|Default|GetEnemyUI) :Type 2)
  (Development|SetHiddeninGame (Variables|Default|GetAttackRange) true false))

(event EventDisableAttack
  ;[1 1 1] AttackSprite
  (|CallParentFunction)
  (Default|SetReaction :self (Variables|Default|GetEnemyUI) :Type 2)
  (Development|SetHiddeninGame (Variables|Default|GetAttackRange) true false))

(event EventSpriteEvent
  ;[1 1 1] AttackSprite
  (Default|SetReaction (Variables|Default|GetEnemyUI) (Variables|Default|GetNextAttackSprite) (Variables|Default|GetReactionColor) 1)
  (Rendering|Material|SetVectorParameterValueonMaterials (Variables|Default|GetAttackRange) "AOEColor" (Math|Conversions|ToVector(LinearColor) "(R=0.604167,G=0.004531,B=0.000000,A=1.000000)")))

(event EventAnimEvent
  ;[1 1 1] AttackSprite
  (Animation|Montage|PlayMontage (Variables|Character|GetMesh) (Variables|Default|GetatkAnim)))

(event EventTick
  (params (DeltaSeconds :type Float%20%28single-precision%29))
  ;[1 1 1] Tick
  (|CallParentFunction DeltaSeconds))

(event EventDealDamages
  (params (attacker :type Actor%20Object%20Reference) (rawDamages :type Float%20%28single-precision%29))
  ;[1 1 1] HitEffects
  (|CallParentFunction attacker rawDamages)
  (CallFunction|AttackedCallback 1.0 1.2)
  (bind _returnvalue (Class|BaseEnemy|GetControllerVibrationfromHit rawDamages (Variables|Default|GetMinControllerVibration) (Variables|Default|GetMaxControllerVibration)))
  (Game|Feedback|PlayDynamicForceFeedback (Game|GetPlayerController 0) _returnvalue (Variables|Default|GetHitVibrationDur) true true true true)
  (bind _asbp_bim_ball_character (Utilities|Casting|CastToBP_BimBallCharacter (Game|GetPlayerCharacter 0)))
  (Utilities|Array|Shuffle (Variables|/Game/Blueprints/Entity/Player/BP_BimBallCharacter.BP_BimBallCharacter_C|GetHitSounds _asbp_bim_ball_character))
  (Audio|PlaySoundatLocation (Utilities|Array|Get(acopy) (Variables|/Game/Blueprints/Entity/Player/BP_BimBallCharacter.BP_BimBallCharacter_C|GetHitSounds _asbp_bim_ball_character)) (Transformation|GetActorLocation) "0, 0, 0" 0.2 1.0 0.0 0 0 0))

(event EventStartAttack
  (params (playerChar_ :type Bim%20Ball%20Character%20Object%20Reference))
  ;[1 1 1] AttackSprite
  (|CallParentFunction playerChar_)
  (Development|SetHiddeninGame (Variables|Default|GetAttackRange) false false)
  (Rendering|Material|SetVectorParameterValueonMaterials (Variables|Default|GetAttackRange) "AOEColor" (Math|Conversions|ToVector(LinearColor) "(R=1.000000,G=0.355562,B=0.281250,A=1.000000)"))
  (Default|SetReaction (Variables|Default|GetEnemyUI) (Variables|Default|GetAttackSprite)))

(event EventBall
  (params (b :type Ball%20Object%20Reference))
  ;[1 1 1] BallSteal
  (|CallParentFunction b)
  (bind _asbp_enemy_controller (Utilities|Casting|CastToBP_EnemyController (AI|GetAIController self)))
  (if (not (Class|EnemyController|DidEnemiesStoleBall _asbp_enemy_controller))
    (bind _asbp_bim_ball_character (Utilities|Casting|CastToBP_BimBallCharacter (Game|GetPlayerCharacter 0)))
    (Default|BallSteal _asbp_bim_ball_character)))

(event EventOnBallHit
  (params (hitBall :type Ball%20Object%20Reference))
  (bind _returnvalue (Transformation|GetActorLocation))
  (bind _bouncesoundvolume (Variables|Default|GetBounceSoundVolume))
  (bind _ballhitslowmo (Variables|Default|GetBallHitSlowMo))
  (bind _ballhitscreenshake (Variables|Default|GetBallHitScreenShake))
  (bind _ballhitvibration (Variables|Default|GetBallHitVibration))
  (bind _enemysoundvolume (Variables|Default|GetEnemySoundVolume))
  (bind (_lerpduration _amount _affectduration _lerpcurve _startupdelay) (Utilities|Struct|BreakBP_SlowMoStruct _ballhitslowmo))
  (bind (_intensity _multipleshakesduration _shaketype _lerpduration_2 _repositionmentdelay _startupdelay_2) (Utilities|Struct|BreakBP_ScreenShakeStruct _ballhitscreenshake))
  (bind (_intensity_2 _duration) (Utilities|Struct|BreakBP_VibrationStruct _ballhitvibration))
  (bind (_min _max) (Utilities|Struct|BreakBP_RandomSoundStruct _bouncesoundvolume))
  (bind (_min_2 _max_2) (Utilities|Struct|BreakBP_RandomSoundStruct _enemysoundvolume))
  ;[1 1 1] OnBallHit
  (|CallParentFunction hitBall)
  (bind _asbp_bim_ball_character (Utilities|Casting|CastToBP_BimBallCharacter (Game|GetPlayerCharacter 0)))
  (Default|Screenshake _asbp_bim_ball_character _intensity _multipleshakesduration _shaketype _lerpduration_2 _repositionmentdelay _startupdelay_2)
  (Game|Feedback|PlayDynamicForceFeedback (Game|GetPlayerController 0) _intensity_2 _duration true true true true)
  (Default|SlowMo _asbp_bim_ball_character _lerpduration _amount _affectduration _lerpcurve _startupdelay)
  (bind _asbp_bim_ball_character_2 (Utilities|Casting|CastToBP_BimBallCharacter (Game|GetPlayerCharacter 0)))
  (Utilities|FlowControl|Sequence
    (:then_0
      (Utilities|Array|Shuffle (Variables|/Game/Blueprints/Props/Ball/BP_Ball.BP_Ball_C|GetBounceSound (Variables|/Game/Blueprints/Entity/Player/BP_BimBallCharacter.BP_BimBallCharacter_C|GetGiveBallReference _asbp_bim_ball_character_2)))
      (Audio|PlaySoundatLocation (Utilities|Array|Get(acopy) (Variables|/Game/Blueprints/Props/Ball/BP_Ball.BP_Ball_C|GetBounceSound (Variables|/Game/Blueprints/Entity/Player/BP_BimBallCharacter.BP_BimBallCharacter_C|GetGiveBallReference _asbp_bim_ball_character_2))) _returnvalue "0, 0, 0" (Math|Random|RandomFloatinRange _min _max) 1.0 0.0 "/Game/SFX/Attenuation/GlobalAttenuation.GlobalAttenuation" 0 0))
    (:then_1
      (Utilities|Array|Shuffle (Variables|/Game/Blueprints/Entity/Player/BP_BimBallCharacter.BP_BimBallCharacter_C|GetEnemyDamageSounds _asbp_bim_ball_character_2))
      (Audio|PlaySoundatLocation (Utilities|Array|Get(acopy) (Variables|/Game/Blueprints/Entity/Player/BP_BimBallCharacter.BP_BimBallCharacter_C|GetEnemyDamageSounds _asbp_bim_ball_character_2)) _returnvalue "0, 0, 0" (Math|Random|RandomFloatinRange _min_2 _max_2) 1.0 0.0 "/Game/SFX/Attenuation/GlobalAttenuation.GlobalAttenuation" 0 0))))

(event EventSetVulnerable
  (bind _vulnerableaoe (Variables|Default|GetVulnerableAOE))
  ;[1 1 1] Vulnerable
  (|CallParentFunction)
  (Utilities|VulnerableCallback
    (:Vulnerable
      (Components|Timeline|SetPlayRate (Variables|Default|GetVulnerableAOEGrowth) 8.0)
      (bind _scale (Timeline|VulnerableAOEGrowth PlayFromStart)
        (:Update
          (Utilities|IsValid _vulnerableaoe
            (:Is%20Valid
              (Transformation|SetRelativeScale3D _vulnerableaoe (Math|Vector|MakeVector (* _scale (Variables|Default|GetVulnerableAOEScale)) (* _scale (Variables|Default|GetVulnerableAOEScale)) (* _scale (Variables|Default|GetVulnerableAOEScale)))))))))
    (:NotVulnerable
      (Timeline|VulnerableAOEGrowth ReverseFromEnd))))

(event EventResetVulnerable
  (bind _vulnerableaoe (Variables|Default|GetVulnerableAOE))
  ;[1 1 1] Vulnerable
  (|CallParentFunction)
  (Utilities|VulnerableCallback) ; enters at ResetVulnerable
)

(fn ConstructionScript)

(fn AttackedCallback
  (params (MinImpactScale :type Float%20%28single-precision%29) (MaxImpactScale :type Float%20%28single-precision%29))
  (bind _returnvalue (Math|Random|RandomFloatinRange MinImpactScale MaxImpactScale))
  (Effects|SpawnEmitterAttached "/Game/VFX/P_AttackImpact_I.P_AttackImpact_I" (Variables|Default|GetCapsuleComponent) "None" "0.000000,0.000000,20.000000" "0, 0, 0" (Math|Vector|MakeVector _returnvalue _returnvalue _returnvalue)))