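; Kamikaze enemy Blueprint that layers visual, audio and UI feedback over its parent's combat events, with a random skeletal mesh per spawn.
; A self-retriggering FlipFlop timeline pulses the warning light alongside a ticking sound until the vulnerable state stops it, recolors the body and grows an AOE indicator.
; Attack events drive range color, explosion sound and reaction sprites.
; Hits add impact particles, rumble and sound, while death destroys the feedback components.
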(event Custom|BlinkLight
  (bind _blinkinglight (Variables|Default|GetBlinkingLight))
  (bind _lightblinking (Variables|Default|GetLightBlinking))
  (bind _explosiontick (Variables|Default|GetExplosionTick))
  (bind _explosiontick_2 (Variables|Default|GetExplosionTick))
  ;[1 1 1] BlinkingLight
  (if (Variables|Default|GetCanBlink) :!label _label
    (Utilities|FlowControl|Sequence
      (:then_0
        (Utilities|IsValid _lightblinking
          (:Is%20Valid
            (Components|Timeline|SetPlayRate _lightblinking (Variables|Default|GetBlinkingRate))
            (Utilities|FlowControl|FlipFlop
              (:A
                (bind _lightintensity (Timeline|LightBlinking PlayFromStart)
                  (:Update
                    (Utilities|IsValid _blinkinglight
                      (:Is%20Valid
                        (Rendering|Components|Light|SetIntensity _blinkinglight (* _lightintensity (Variables|Default|GetBlinkIntensityMultiplier))))))
                  (:Finished
                    (goto _label))))
              (:B
                (Timeline|LightBlinking ReverseFromEnd))))))
      (:then_1
        (Utilities|IsValid _explosiontick
          (:Is%20Valid
            (Audio|Components|Audio|SetSound _explosiontick "/Game/SFX/SoundWave_SFX/Kamikaze_Run_01.Kamikaze_Run_01")
            (Audio|Components|Audio|Play _explosiontick 0.0)))))
    (else
      (Utilities|IsValid _explosiontick_2
        (:Is%20Valid
          (Audio|Components|Audio|Stop _explosiontick_2))))))

(event Custom|StopLight
  (bind _blinkinglight (Variables|Default|GetBlinkingLight))
  (bind _lightblinking (Variables|Default|GetLightBlinking))
  (bind _explosiontick (Variables|Default|GetExplosionTick))
  (bind _explosiontick_2 (Variables|Default|GetExplosionTick))
  ;[1 1 1] BlinkingLight
  (bind _lightintensity (Timeline|LightBlinking Stop)
    (:Update
      (Utilities|IsValid _blinkinglight
        (:Is%20Valid
          (Rendering|Components|Light|SetIntensity _blinkinglight (* _lightintensity (Variables|Default|GetBlinkIntensityMultiplier))))))
    (:Finished
      (if (Variables|Default|GetCanBlink)
        (Utilities|FlowControl|Sequence
          (:then_0
            (Utilities|IsValid _lightblinking
              (:Is%20Valid
                (Components|Timeline|SetPlayRate _lightblinking (Variables|Default|GetBlinkingRate))
                (Utilities|FlowControl|FlipFlop
                  (:A
                    (Timeline|LightBlinking PlayFromStart))
                  (:B
                    (Timeline|LightBlinking ReverseFromEnd))))))
          (:then_1
            (Utilities|IsValid _explosiontick
              (:Is%20Valid
                (Audio|Components|Audio|SetSound _explosiontick "/Game/SFX/SoundWave_SFX/Kamikaze_Run_01.Kamikaze_Run_01")
                (Audio|Components|Audio|Play _explosiontick 0.0)))))
        (else
          (Utilities|IsValid _explosiontick_2
            (:Is%20Valid
              (Audio|Components|Audio|Stop _explosiontick_2))))))))

(event EventOnHpZero
  (params (killer :type Actor%20Object%20Reference))
  ;[1 1 1] DeathFX
  (|CallParentFunction killer)
  (Utilities|FlowControl|Sequence
    (:then_0
      (CallFunction|AttackedCallback 2.8 3.0)
      (CallFunction|StopLight))
    (:then_1
      (Components|DestroyComponent (Variables|Default|GetLightBlinking))
      (Components|DestroyComponent (Variables|Default|GetVulnerableAOEGrowth))
      (Components|DestroyComponent (Variables|Default|GetAttackRange))
      (Components|DestroyComponent (Variables|Default|GetUI))
      (Components|DestroyComponent (Variables|Default|GetVulnerableAOE))
      (Components|DestroyComponent (Variables|Default|GetBlinkingLight))
      (Components|DestroyComponent (Variables|Default|GetExplosionTick)))))

(event EventSpriteEvent
  (bind _explosiontick (Variables|Default|GetExplosionTick))
  ;[1 1 1] AttackSprite
  (Audio|Components|Audio|SetSound _explosiontick (Variables|Default|GetExplosionSound))
  (Audio|Components|Audio|Play _explosiontick 0.0)
  (Rendering|Material|SetVectorParameterValueonMaterials (Variables|Default|GetAttackRange) "AOEColor" (Math|Conversions|ToVector(LinearColor) "(R=0.604167,G=0.004531,B=0.000000,A=1.000000)"))
  (Default|SetReaction :self (Variables|Default|GetEnemyUI) :Brush (Variables|Default|GetExplosionSprite) :Type 1))

(event EventTick
  (params (DeltaSeconds :type Float%20%28single-precision%29))
  ;[1 1 1] Tick
  (|CallParentFunction DeltaSeconds))

(event EventDealDamages
  (params (attacker :type Actor%20Object%20Reference) (rawDamages :type Float%20%28single-precision%29))
  ;[1 1 1] HitEffects
  (|CallParentFunction attacker rawDamages)
  (CallFunction|AttackedCallback 1.0 1.2)
  (bind _returnvalue (Class|BaseEnemy|GetControllerVibrationfromHit 0.0 (Variables|Default|GetMinControllerVibration) (Variables|Default|GetMaxControllerVibration)))
  (Game|Feedback|PlayDynamicForceFeedback (Game|GetPlayerController 0) _returnvalue (Variables|Default|GetHitVibrationDur) true true true true)
  (bind _asbp_bim_ball_character (Utilities|Casting|CastToBP_BimBallCharacter (Game|GetPlayerCharacter 0)))
  (Utilities|Array|Shuffle (Variables|/Game/Blueprints/Entity/Player/BP_BimBallCharacter.BP_BimBallCharacter_C|GetHitSounds _asbp_bim_ball_character))
  (Audio|PlaySoundatLocation (Utilities|Array|Get(acopy) (Variables|/Game/Blueprints/Entity/Player/BP_BimBallCharacter.BP_BimBallCharacter_C|GetHitSounds _asbp_bim_ball_character)) (Transformation|GetActorLocation) "0, 0, 0" 0.6 1.0 0.0 "/Game/SFX/Attenuation/GlobalAttenuation.GlobalAttenuation" 0 0))

(event EventStartAttack
  (params (playerChar_ :type Bim%20Ball%20Character%20Object%20Reference))
  (bind _attackrange (Variables|Default|GetAttackRange))
  ;[1 1 1] AttackSprite
  (|CallParentFunction playerChar_)
  (Development|SetHiddeninGame _attackrange false false)
  (Rendering|Material|SetVectorParameterValueonMaterials _attackrange "AOEColor" (Math|Conversions|ToVector(LinearColor) "(R=1.000000,G=0.355562,B=0.281250,A=1.000000)"))
  (Default|SetReaction (Variables|Default|GetEnemyUI) (Variables|Default|GetAttackSprite)))

(event EventDisableAttack
  (bind _attackrange (Variables|Default|GetAttackRange))
  (bind _enemyui (Variables|Default|GetEnemyUI))
  ;[1 1 1] AttackSprite
  (|CallParentFunction)
  (Utilities|IsValid _enemyui
    (:Is%20Valid
      (Default|SetReaction :self _enemyui :Type 2)
      (Utilities|IsValid _attackrange
        (:Is%20Valid
          (Development|SetHiddeninGame _attackrange true false))))))

(event EventBeginPlay
  ;[1 1 1] BeginPlay
  (|CallParentFunction)
  (Utilities|FlowControl|Sequence
    (:then_0
      (bind _asbp_enemy_ui (Utilities|Casting|CastToBP_EnemyUI (Variables|/Script/Engine.ChildActorComponent|GetChildActor (Variables|Default|GetUI))))
      (Variables|Default|SetEnemyUI _asbp_enemy_ui)
      (Class|SkinnedMeshComponent|SetSkeletalMesh (Variables|Character|GetMesh) (Utilities|Select :Index (Math|Random|RandomIntegerinRange 0 2) :Option%200 "/Game/Meshes/ModularRPGHeroesPolyart/OneMeshCharacters/SK_Shinobi.SK_Shinobi" :Option%201 "/Game/Meshes/ModularRPGHeroesPolyart/OneMeshCharacters/TemplarSK.TemplarSK" :Option%202 "/Game/Meshes/ModularRPGHeroesPolyart/OneMeshCharacters/SK_Engineer.SK_Engineer") false)
      (Class|BaseEnemy|ResetVulnerable))
    (:then_1
      (CallFunction|BlinkLight))))

(event EventSetVulnerable
  (bind _vulnerableaoe (Variables|Default|GetVulnerableAOE))
  ;[1 1 1] Vulnerable
  (|CallParentFunction)
  (Utilities|VulnerableCallback
    (:Vulnerable
      (CallFunction|StopLight)
      (Rendering|Components|Light|SetIntensity (Variables|Default|GetBlinkingLight) 0.0)
      (Components|Timeline|SetPlayRate (Variables|Default|GetVulnerableAOEGrowth) 8.0)
      (bind _scale (Timeline|VulnerableAOEGrowth PlayFromStart)
        (:Update
          (Utilities|IsValid _vulnerableaoe
            (:Is%20Valid
              (Transformation|SetRelativeScale3D _vulnerableaoe (Math|Vector|MakeVector (* _scale (Variables|Default|GetVulnerableAOEScale)) (* _scale (Variables|Default|GetVulnerableAOEScale)) (* _scale (Variables|Default|GetVulnerableAOEScale)))))))))
    (:NotVulnerable
      (CallFunction|BlinkLight)
      (Timeline|VulnerableAOEGrowth ReverseFromEnd))))

(event EventResetVulnerable
  (bind _vulnerableaoe (Variables|Default|GetVulnerableAOE))
  ;[1 1 1] Vulnerable
  (|CallParentFunction)
  (Utilities|VulnerableCallback) ; enters at ResetVulnerable
)

(fn ConstructionScript)

(fn AttackedCallback
  (params (minImpactScale :type Float%20%28single-precision%29) (maxImpactScale :type Float%20%28single-precision%29))
  (bind _returnvalue (Math|Random|RandomFloatinRange minImpactScale maxImpactScale))
  (Effects|SpawnEmitterAttached "/Game/VFX/P_AttackImpact_I.P_AttackImpact_I" (Variables|Default|GetCapsuleComponent) "None" "0.000000,0.000000,20.000000" "0, 0, 0" (Math|Vector|MakeVector _returnvalue _returnvalue _returnvalue)))