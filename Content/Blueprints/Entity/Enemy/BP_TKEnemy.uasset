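; Tackling enemy in the BimBall game that layers presentation and feedback over its parent enemy's combat events.
; Basic attacks and tackles drive the reaction UI, montages and AOE indicators, with tackles adding sounds, a timeline-grown AOE and a forward snap.
; Vulnerability toggles a fresnel highlight and scaled AOE via a macro.
; Hits spawn impact effects and sounds, ball hits add player screenshake, rumble and slow-mo, and ball steals notify the player.
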(event Custom|TackleSprite
  (bind _tackleaoe (Variables|Default|GetTackleAOE))
  (bind _tackleaoegrowth (Variables|Default|GetTackleAOEGrowth))
  (bind _tacklesounds (Variables|Default|GetTackleSounds))
  ;[1 1 1] Attack
  ;;[1 1 1] Tackle
  (Default|SetReaction :self (Variables|Default|GetEnemyUI) :Brush (Variables|Default|GetnextChargeSprite) :Type 1)
  (Audio|Components|Audio|SetSound _tacklesounds "/Game/SFX/SoundWave_SFX/ChargeTackler.ChargeTackler")
  (Audio|Components|Audio|Play _tacklesounds 0.0)
  (Development|SetHiddeninGame (Variables|Default|GetTackleAOE) false false)
  (Components|Timeline|SetPlayRate _tackleaoegrowth (/ (Components|Timeline|GetTimelineLength _tackleaoegrowth) (Variables|Default|GetAOEGrowthDuration)))
  (bind _aoescalex (Timeline|TackleAOEGrowth PlayFromStart)
    (:Update
      (Utilities|IsValid _tackleaoe
        (:Is%20Valid
          (Transformation|SetRelativeTransform _tackleaoe (Math|Transform|MakeTransform (Math|Vector|MakeVector (* _aoescalex (Variables|Default|GetAOEoffset)) 0.0 -89.0) "0, 0, 0" (Math|Vector|MakeVector (* _aoescalex (Variables|Default|GetAOEMaxScaleX)) 7.5 1.0)) false false))))))

(event Custom|BasicAttackSprite
  ;[1 1 1] Attack
  ;;[1 1 1] BasicAttack
  (Default|SetReaction (Variables|Default|GetEnemyUI) (Variables|Default|GetnextAtkSprite) (Variables|Default|GetReactionColor) 1)
  (Rendering|Material|SetVectorParameterValueonMaterials (Variables|Default|GetAttackRange) "AOEColor" (Math|Conversions|ToVector(LinearColor) "(R=0.604167,G=0.004531,B=0.000000,A=1.000000)")))

(event EventBeginPlay
  ;[1 1 1] BeginPlay
  (|CallParentFunction)
  (bind _asbp_enemy_ui (Utilities|Casting|CastToBP_EnemyUI (Variables|/Script/Engine.ChildActorComponent|GetChildActor (Variables|Default|GetUI))))
  (Variables|Default|SetEnemyUI _asbp_enemy_ui)
  (Class|BaseEnemy|ResetVulnerable))

(event EventOnHpZero
  (params (killer :type Actor%20Object%20Reference))
  ;[1 1 1] DeathFX
  (|CallParentFunction killer)
  (CallFunction|AttackedCallback 2.8 3.0)
  (Components|DestroyComponent (Variables|Default|GetVulnerableAOEGrowth))
  (Components|DestroyComponent (Variables|Default|GetTackleAOEGrowth))
  (Components|DestroyComponent (Variables|Default|GetUI))
  (Components|DestroyComponent (Variables|Default|GetTackleAOE))
  (Components|DestroyComponent (Variables|Default|GetVulnerableAOE))
  (Components|DestroyComponent (Variables|Default|GetAttackRange)))

(event EventResetVulnerable
  (bind _vulnerableaoe (Variables|Default|GetVulnerableAOE))
  ;[1 1 1] Vulnerable Material
  (|CallParentFunction)
  (Utilities|VulnerableCallback) ; enters at ResetVulnerable
)

(event EventAttack
  (params (playerChar_ :type Bim%20Ball%20Character%20Object%20Reference))
  ;[1 1 1] Attack
  ;;[1 1 1] Tackle
  (Utilities|FlowControl|Sequence
    (:then_0
      (Audio|Components|Audio|Stop (Variables|Default|GetTackleSounds))
      (if (Variables|Default|GetisTackling)
        (Class|Entity|SnaptoLocation (|(loc+(forward*length)) (Transformation|GetActorLocation) (Transformation|GetActorForwardVector) 5e+02))
        (Animation|Montage|PlayMontage (Variables|Character|GetMesh) (Variables|Default|GettackleAnim))))
    (:then_1
      (|CallParentFunction playerChar_))))

(event EventSpriteEvent
  ;[1 1 1] Attack
  ;;[1 1 1] Chose AttackSprite
  (if (Variables|Default|GetisTackling)
    (CallFunction|TackleSprite)
    (else
      (CallFunction|BasicAttackSprite))))

(event EventAnimEvent
  ;[1 1 1] Attack
  ;;[1 1 1] BasicAttack
  (if (not (Variables|Default|GetisTackling))
    (Animation|Montage|PlayMontage (Variables|Character|GetMesh) (Variables|Default|GetbaseAtkAnim))))

(event EventTick
  (params (DeltaSeconds :type Float%20%28single-precision%29))
  ;[1 1 1] Tick
  (|CallParentFunction DeltaSeconds))

(event EventDealDamages
  (params (attacker :type Actor%20Object%20Reference) (rawDamages :type Float%20%28single-precision%29))
  ;[1 1 1] HitEffects
  (|CallParentFunction attacker rawDamages)
  (CallFunction|AttackedCallback 1.0 1.2)
  (bind _asbp_bim_ball_character (Utilities|Casting|CastToBP_BimBallCharacter (Game|GetPlayerCharacter 0)))
  (Utilities|Array|Shuffle (Variables|/Game/Blueprints/Entity/Player/BP_BimBallCharacter.BP_BimBallCharacter_C|GetHitSounds _asbp_bim_ball_character))
  (Audio|PlaySoundatLocation (Utilities|Array|Get(acopy) (Variables|/Game/Blueprints/Entity/Player/BP_BimBallCharacter.BP_BimBallCharacter_C|GetHitSounds _asbp_bim_ball_character)) (Transformation|GetActorLocation) "0, 0, 0" 0.2 1.0 0.0 0 0 0))

(event EventStartAttack
  (params (playerChar_ :type Bim%20Ball%20Character%20Object%20Reference))
  ;[1 1 1] Attack
  ;;[1 1 1] BasicAttack
  (|CallParentFunction playerChar_)
  (Development|SetHiddeninGame (Variables|Default|GetAttackRange) false false)
  (Rendering|Material|SetVectorParameterValueonMaterials (Variables|Default|GetAttackRange) "AOEColor" (Math|Conversions|ToVector(LinearColor) "(R=1.000000,G=0.355562,B=0.281250,A=1.000000)"))
  (Default|SetReaction (Variables|Default|GetEnemyUI) (Variables|Default|GetAttackSprite)))

(event EventBall
  (params (b :type Ball%20Object%20Reference))
  ;[1 1 1] BallSteal
  (|CallParentFunction b)
  (bind _asbp_enemy_controller (Utilities|Casting|CastToBP_EnemyController (AI|GetAIController self)))
  (if (not (Class|EnemyController|DidEnemiesStoleBall _asbp_enemy_controller))
    (bind _asbp_bim_ball_character (Utilities|Casting|CastToBP_BimBallCharacter (Game|GetPlayerCharacter 0)))
    (Default|BallSteal _asbp_bim_ball_character)))

(event EventDisableAttack
  ;[1 1 1] Attack
  ;;[1 1 1] EndAttack
  (|CallParentFunction)
  (Audio|Components|Audio|Stop (Variables|Default|GetTackleSounds))
  (Default|SetReaction :self (Variables|Default|GetEnemyUI) :Type 2)
  (Development|SetHiddeninGame (Variables|Default|GetAttackRange) true false)
  (Development|SetHiddeninGame (Variables|Default|GetTackleAOE) true false))

(event EventOnBallHit
  (params (hitBall :type Ball%20Object%20Reference))
  (bind _returnvalue (Transformation|GetActorLocation))
  (bind _ballhitslowmo (Variables|Default|GetBallHitSlowMo))
  (bind _ballhitvibration (Variables|Default|GetBallHitVibration))
  (bind _bouncesoundvolume (Variables|Default|GetBounceSoundVolume))
  (bind _enemysoundvolume (Variables|Default|GetEnemySoundVolume))
  (bind _ballhitscreenshake (Variables|Default|GetBallHitScreenShake))
  (bind (_intensity _multipleshakesduration _shaketype _lerpduration _repositionmentdelay _startupdelay) (Utilities|Struct|BreakBP_ScreenShakeStruct _ballhitscreenshake))
  (bind (_lerpduration_2 _amount _affectduration _lerpcurve _startupdelay_2) (Utilities|Struct|BreakBP_SlowMoStruct _ballhitslowmo))
  (bind (_intensity_2 _duration) (Utilities|Struct|BreakBP_VibrationStruct _ballhitvibration))
  (bind (_min _max) (Utilities|Struct|BreakBP_RandomSoundStruct _bouncesoundvolume))
  (bind (_min_2 _max_2) (Utilities|Struct|BreakBP_RandomSoundStruct _enemysoundvolume))
  ;[1 1 1] OnBallHit
  (|CallParentFunction hitBall)
  (bind _asbp_bim_ball_character (Utilities|Casting|CastToBP_BimBallCharacter (Game|GetPlayerCharacter 0)))
  (Default|Screenshake _asbp_bim_ball_character _intensity _multipleshakesduration _shaketype _lerpduration _repositionmentdelay _startupdelay)
  (Game|Feedback|PlayDynamicForceFeedback (Game|GetPlayerController 0) _intensity_2 _duration true true true true)
  (Default|SlowMo _asbp_bim_ball_character _lerpduration_2 _amount _affectduration _lerpcurve _startupdelay_2)
  (bind _asbp_bim_ball_character_2 (Utilities|Casting|CastToBP_BimBallCharacter (Game|GetPlayerCharacter 0)))
  (Utilities|FlowControl|Sequence
    (:then_0
      (Utilities|Array|Shuffle (Variables|/Game/Blueprints/Props/Ball/BP_Ball.BP_Ball_C|GetBounceSound (Variables|/Game/Blueprints/Entity/Player/BP_BimBallCharacter.BP_BimBallCharacter_C|GetGiveBallReference _asbp_bim_ball_character_2)))
      (Audio|PlaySoundatLocation (Utilities|Array|Get(acopy) (Variables|/Game/Blueprints/Props/Ball/BP_Ball.BP_Ball_C|GetBounceSound (Variables|/Game/Blueprints/Entity/Player/BP_BimBallCharacter.BP_BimBallCharacter_C|GetGiveBallReference _asbp_bim_ball_character_2))) _returnvalue "0, 0, 0" (Math|Random|RandomFloatinRange _min _max) 1.0 0.0 "/Game/SFX/Attenuation/GlobalAttenuation.GlobalAttenuation" 0 0))
    (:then_1
      (Utilities|Array|Shuffle (Variables|/Game/Blueprints/Entity/Player/BP_BimBallCharacter.BP_BimBallCharacter_C|GetEnemyDamageSounds _asbp_bim_ball_character_2))
      (Audio|PlaySoundatLocation (Utilities|Array|Get(acopy) (Variables|/Game/Blueprints/Entity/Player/BP_BimBallCharacter.BP_BimBallCharacter_C|GetEnemyDamageSounds _asbp_bim_ball_character_2)) _returnvalue "0, 0, 0" (Math|Random|RandomFloatinRange _min_2 _max_2) 1.0 0.0 "/Game/SFX/Attenuation/GlobalAttenuation.GlobalAttenuation" 0 0))))

(event EventStartTackle
  (bind _tacklesounds (Variables|Default|GetTackleSounds))
  ;[1 1 1] Attack
  ;;[1 1 1] Tackle
  (|CallParentFunction)
  (Default|SetReaction (Variables|Default|GetEnemyUI) (Variables|Default|GetChargeSprite))
  (Audio|Components|Audio|SetSound _tacklesounds "/Game/SFX/SoundWave_SFX/InitTackler.InitTackler")
  (Audio|Components|Audio|Play _tacklesounds 0.0))

(event EventSetVulnerable
  (bind _vulnerableaoe (Variables|Default|GetVulnerableAOE))
  ;[1 1 1] Vulnerable Material
  (|CallParentFunction)
  (Utilities|VulnerableCallback
    (:Vulnerable
      (Components|Timeline|SetPlayRate (Variables|Default|GetVulnerableAOEGrowth) 8.0)
      (bind _scale (Timeline|VulnerableAOEGrowth PlayFromStart)
        (:Update
          (Utilities|IsValid _vulnerableaoe
            (:Is%20Valid
              (Transformation|SetRelativeScale3D _vulnerableaoe (Math|Vector|MakeVector (* _scale (Variables|Default|GetVulnerableAOEScale)) (* _scale (Variables|Default|GetVulnerableAOEScale)) (* _scale (Variables|Default|GetVulnerableAOEScale)))))))))
    (:NotVulnerable
      (Timeline|VulnerableAOEGrowth ReverseFromEnd))))

(fn ConstructionScript)

(fn AttackedCallback
  (params (Min :type Float%20%28single-precision%29) (Max :type Float%20%28single-precision%29))
  (bind _returnvalue (Math|Random|RandomFloatinRange Min Max))
  (Effects|SpawnEmitterAttached "/Game/VFX/P_AttackImpact_I.P_AttackImpact_I" (Variables|Default|GetCapsuleComponent) "None" "0.000000,0.000000,20.000000" "0, 0, 0" (Math|Vector|MakeVector _returnvalue _returnvalue _returnvalue)))