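; BP_Ball is the BimBall ball, handling its indicators and charge feedback, and registering itself with the player character on BeginPlay.
; Tick updates ground and see-through indicators, computes screen-edge arrow position when off-screen, and shows a camera-facing rush prompt when rush is available.
; See-through swaps the ball material and attaches a spawned indicator actor.
; Aim and charge events drive audio, particles and material parameters.
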(event Custom|OnCharged
  (bind _ballchargeaudio (Variables|Default|GetBallChargeAudio))
  (bind _ballmesh (Variables|Default|GetballMesh))
  ;[1 1 1] BallCharged
  (Audio|PlaySoundatLocation "/Game/SFX/SoundWave_SFX/ChargedBeep.ChargedBeep" (Transformation|GetActorLocation) "0, 0, 0" 1.5 1.0 0.0 0 0 0)
  (Rendering|Material|SetScalarParameterValueonMaterials _ballmesh "BallCharged" 1.0)
  (Rendering|Material|SetScalarParameterValueonMaterials _ballmesh "FresnelPower" 4.5)
  (Audio|Components|Audio|SetSound _ballchargeaudio "/Game/SFX/SoundWave_SFX/ChargedLoop.ChargedLoop")
  (Audio|Components|Audio|Play _ballchargeaudio 0.0)
  (bind _returnvalue (Effects|SpawnEmitteratLocation "/Game/VFX/P_BallCharged.P_BallCharged" (Transformation|GetActorLocation))))

(event Custom|OnUncharged
  (bind _ballmesh (Variables|Default|GetballMesh))
  ;[1 1 1] BallCharged
  (Rendering|Material|SetScalarParameterValueonMaterials _ballmesh "BallCharged" 0.0)
  (Rendering|Material|SetScalarParameterValueonMaterials _ballmesh "FresnelPower" 7.0)
  (Utilities|IsValid (stale Custom|OnCharged _returnvalue)
    (:Is%20Valid
      (Components|DestroyComponent (stale Custom|OnCharged _returnvalue)))))

(event Custom|OnAimEnd
  ;[1 1 1] BallCharging
  (Utilities|IsValid (stale Custom|OnAimStart _returnvalue)
    (:Is%20Valid
      (Audio|Components|Audio|Stop (Variables|Default|GetBallChargeAudio))
      (Components|DestroyComponent (stale Custom|OnAimStart _returnvalue)))))

(event Custom|OnAimStart
  (bind _ballchargeaudio (Variables|Default|GetBallChargeAudio))
  ;[1 1 1] BallCharging
  (Audio|Components|Audio|SetSound _ballchargeaudio "/Game/SFX/SoundWave_SFX/ChargeUp.ChargeUp")
  (Audio|Components|Audio|Play _ballchargeaudio 0.0)
  (bind _returnvalue (Effects|SpawnEmitterAttached "/Game/VFX/P_BallCharging.P_BallCharging" (Variables|Default|GetballMesh) "None")))

(event EventEnableBallSeeThrough
  ;[1 1 1] Ball Seethrough Activation
  (|CallParentFunction)
  (Rendering|Material|SetMaterial (Variables|Default|GetballMesh) 0 (Variables|Default|GetSeeThroughMaterial))
  (bind _returnvalue (Game|SpawnActorfromClass "/Game/Blueprints/UI/InGame/Ball/BP_BallSeeThrough.BP_BallSeeThrough_C" (Transformation|GetActorTransform) "Undefined" 0 0))
  (bind _output_get (Variables|Default|SetSeeThroughIndicator _returnvalue))
  (Transformation|AttachActorToActor _output_get self "None" "SnapToTarget" "KeepWorld" "KeepRelative" true))

(event EventTick
  (params (DeltaSeconds :type Float%20%28single-precision%29))
  ;[1 1 1] Tick
  (|CallParentFunction DeltaSeconds)
  (Utilities|FlowControl|Sequence
    (:then_0
      (Class|Ball|UpdateGroundIndicator (Variables|Default|GetballPositionPlaceholder) "ECC_GameTraceChannel1"))
    (:then_1
      (Class|Ball|UpdateBallSeeThrough))
    (:then_2
      (CallFunction|UpdateBallArrowIndicator))
    (:then_3
      (CallFunction|UpdateBallrushIndicator))))

(event EventDisableBallSeeThrough
  (bind _seethroughindicator (Variables|Default|GetSeeThroughIndicator))
  ;[1 1 1] Ball Seethrough Activation
  (|CallParentFunction)
  (Rendering|Material|SetMaterial (Variables|Default|GetballMesh) 0 (Variables|Default|GetBallMaterial))
  (if (Utilities|IsValid _seethroughindicator)
    (Actor|DestroyActor _seethroughindicator)))

(event EventBeginPlay
  ;[1 1 1] Why do I have to do this to give a BP_Ball reference to something
  (|CallParentFunction)
  (Utilities|FlowControl|Sequence
    (:then_0
      (bind _asbp_bim_ball_character (Utilities|Casting|CastToBP_BimBallCharacter (Game|GetPlayerCharacter 0)))
      (Default|GiveBallRef _asbp_bim_ball_character self)
      (bind _asbp_bim_ball_game_mode (Utilities|Casting|CastToBP_BimBallGameMode (Game|GetGameMode)))
      (Variables|Default|SetballIndicatorBounds (- (Variables|/Game/Blueprints/GameManagement/BP_BimBallGameMode.BP_BimBallGameMode_C|GetHalfScreenResolution _asbp_bim_ball_game_mode) (Variables|Default|GetballIndicatorOffset))))
    (:then_1
      (bind _asbp_ball_see_through_ui (Utilities|Casting|CastToBP_BallSeeThroughUI (UserInterface|GetUserWidgetObject (Variables|Default|GetBallRushIndicator))))
      (Appearance|SetBrushfromTexture (Variables|/Game/Blueprints/UI/InGame/Ball/BP_BallSeeThroughUI.BP_BallSeeThroughUI_C|GetIndicator _asbp_ball_see_through_ui) (Variables|Default|GetBallRushTexture) false)
      (Class|WidgetComponent|SetTintColorandOpacity (Variables|Default|GetBallRushIndicator) "(R=1.000000,G=0.404574,B=0.000000,A=1.000000)")
      (UserInterface|Animation|PlayAnimation _asbp_ball_see_through_ui (Variables|/Game/Blueprints/UI/InGame/Ball/BP_BallSeeThroughUI.BP_BallSeeThroughUI_C|GetIndicatorRotation _asbp_ball_see_through_ui) 0.0 0 "Forward" (/ (Class|WidgetAnimation|GetEndTime (Variables|/Game/Blueprints/UI/InGame/Ball/BP_BallSeeThroughUI.BP_BallSeeThroughUI_C|GetIndicatorRotation _asbp_ball_see_through_ui)) 2.0) false))))

(fn ConstructionScript)

(fn IsBallRushAvailable
  (params (self2 :type BP%20Bim%20Ball%20Character%20Object%20Reference))
  (return (Math|Boolean|ANDBoolean (<= (Transformation|GetDistanceTo (Game|GetPlayerCharacter 0)) (Variables|/Script/Engine.SphereComponent|GetSphereRadius (Variables|/Script/BimBall.BimBallCharacter|GetballSnapRange self2))) (not (Variables|/Game/Blueprints/Entity/Player/BP_BimBallCharacter.BP_BimBallCharacter_C|GetBallRushCD self2)) (not (Variables|Default|GetisSeeThrough)) (not (Class|Ball|IsinOwnerHands)) (Class|Ball|GetIsTakable))))

(fn UpdateBallrushIndicator
  (bind _ballrushindicator (Variables|Default|GetBallRushIndicator))
  (bind _asbp_bim_ball_character (Utilities|Casting|CastToBP_BimBallCharacter (Game|GetPlayerCharacter 0)))
  (if (CallFunction|IsBallRushAvailable _asbp_bim_ball_character)
    (Development|SetHiddeninGame _ballrushindicator false false)
    (Transformation|SetWorldRotation _ballrushindicator (Math|Rotator|FindLookatRotation (Transformation|GetWorldLocation _ballrushindicator) (Camera|GetCameraLocation (Game|GetPlayerCameraManager 0))) false false)
    (else
      (Development|SetHiddeninGame _ballrushindicator true false))))

(fn UpdateBallArrowIndicator
  (bind (_outputloc _returnvalue) (Class|Ball|ComputeBallScreenLocation))
  (Variables|Default|SetballIndicatorBounds (Class|Ball|ComputeBallIndicatorBounds))
  (bind _output_get (Variables|Default|SetRenderArrowIndicator (not (or (and (== (Variables|Default|GetownerCharacter) (Game|Player|GetPlayerPawn 0)) (Class|Ball|IsinOwnerHands)) (Class|Actor|WasRecentlyRendered self 0.1)))))
  (if _output_get
    (if _returnvalue
      (bind _output_get_2 (Variables|Default|SetBallIndicatorPosition (Class|Ball|ComputeBallIndicatorLocation _outputloc)))
      (Variables|Default|SetBallIndicatorAngle (Class|Ball|ComputeBallIndicatorAngle _output_get_2)))))